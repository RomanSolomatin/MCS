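; Lightsaber weapon actor that extends and retracts a glowing, colored blade with timelines, light, hum, trails and impact effects.
; While hit detection is enabled, Tick runs swept box traces from each blade socket's previous location to its current one, stopping at the first valid hit.
; Saber and character hits are sent to the parent actor through interface messages, and saber contact also disables tracing.
; Debug toggles control trace drawing and hit info.
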(event Custom|Initialize
  ;[1 1 1] Initialize and set references
  (Variables|HitDetection|SetActorsToIgnore (Utilities|Array|MakeArray (Actor|GetParentActor))))

(event Custom|DrawWeapon
  (bind _saberhum (Variables|Weapon|GetSaberHum))
  ;[1 1 1] Turn lightsaber ON/OFF.  Enable/Disable collision respectively.
  (Variables|Weapon|SetInProgress true)
  (Rendering|SetVisibility (Variables|Default|GetHilt) true true)
  (Audio|Components|Audio|SetVolumeMultiplier _saberhum 1.0 :!class /Script/Engine.AudioComponent)
  (Audio|Components|Audio|Play _saberhum 0.0)
  (Audio|PlaySoundatLocation "/Game/MCS/Sounds/Saber/saberon_Cue.SaberOn_Cue" (Transformation|GetActorLocation))
  (bind _bladezlength (Timeline|BladeExtendTime PlayFromStart)
    (:Update
      (Transformation|SetWorldScale3D (Variables|Default|GetBlade) (Math|Vector|MakeVector 1.0 1.0 _bladezlength))
      (Rendering|Components|Light|SetIntensity (Variables|Default|GetBladeLight) (* _bladezlength (Variables|Materials|GetDefaultLightIntesity))))
    (:Finished
      (Variables|Weapon|SetIsWeaponDrawn? true)
      (Weapon|SetCollision true)
      (Variables|Weapon|SetInProgress false))))

(event Custom|GrabHilt
  ;[1 1 1] HACK to grab the hilt (just makes it visible)
  (Rendering|SetVisibility (Variables|Default|GetHilt) true true))

(event Custom|SheathWeapon
  ;[1 1 1] Turn lightsaber ON/OFF.  Enable/Disable collision respectively.
  (Variables|Weapon|SetInProgress true)
  (Audio|PlaySoundatLocation "/Game/MCS/Sounds/Saber/saberoff_Cue.SaberOff_Cue" (Transformation|GetActorLocation))
  (bind _bladezlength (Timeline|BladeContractTime PlayFromStart)
    (:Update
      (Transformation|SetWorldScale3D (Variables|Default|GetBlade) (Math|Vector|MakeVector 1.0 1.0 _bladezlength))
      (Rendering|Components|Light|SetIntensity (Variables|Default|GetBladeLight) (* _bladezlength (Variables|Materials|GetDefaultLightIntesity))))
    (:Finished
      (Audio|Components|Audio|Stop (Variables|Weapon|GetSaberHum))
      (Variables|Weapon|SetIsWeaponDrawn? false)
      (Weapon|SetCollision true)
      (Variables|Weapon|SetInProgress false))))

(event Custom|ToggleWeaponTrails
  (params (Toggle :type Boolean))
  ;[1 1 1] Weapon Trails
  (if (Variables|Weapon|GetShowWeaponTrails)
    (if Toggle
      (Effects|Particles|Trails|BeginTrails (Variables|Default|GetWeaponTrail) "sock_01" "blade_tip" "ETrailWidthMode_FromCentre" 1.0)
      (else
        (Effects|Particles|Trails|EndTrails (Variables|Default|GetWeaponTrail))))))

(event Custom|BladeHitBlade
  (params (HitResult :type Hit%20Result%20Structure%20%28by%20ref%29))
  (bind _impactpoint (Collision|BreakHitResult HitResult))
  ;[1 1 1] Spawn a particle effect at the point of impact
  (Audio|PlaySoundatLocation "/Game/MCS/Sounds/Saber/SaberHits_Cue.SaberHits_Cue" _impactpoint)
  (Effects|SpawnEmitteratLocation "/Game/MCS/ParticleFX/P_SaberImpact.P_SaberImpact" _impactpoint))

(event Custom|UpdateSaberColor
  (params (Color :type Linear%20Color%20Structure))
  (bind _bladematerial (Variables|Materials|GetBladeMaterial))
  ;[1 1 1] Lightsaber blade color
  (bind _output_get (Variables|Materials|SetSaberColor Color))
  (Rendering|Material|SetVectorParameterValue _bladematerial "EmissiveColor" _output_get :!class /Script/Engine.MaterialInstanceDynamic)
  (Rendering|Material|SetVectorParameterValue _bladematerial "EmissiveStrength" "(R=50.000000,G=50.000000,B=50.000000,A=1.000000)" :!class /Script/Engine.MaterialInstanceDynamic)
  (Rendering|Components|Light|SetLightColor (Variables|Default|GetBladeLight) (Variables|Materials|GetSaberColor) true)
  (bind _returnvalue (Rendering|Material|CreateDynamicMaterialInstance (Rendering|Material|GetMaterial (Variables|Default|GetWeaponTrail) 0) "/Game/MCS/Materials/WeaponTrails/MI_WeaponTrail.MI_WeaponTrail" :!class /Script/Engine.KismetMaterialLibrary))
  (Rendering|Material|SetVectorParameterValue _returnvalue "BaseColor" (Variables|Materials|GetSaberColor) :!class /Script/Engine.MaterialInstanceDynamic)
  (Rendering|Material|SetMaterial (Variables|Default|GetWeaponTrail) 0 _returnvalue))

(event Custom|ToggleTraceVisibility
  ;[1 0.8453 0.2404] DEBUG: Toggle trace lines / hit information.
  (switch Utilities|FlowControl|Switch|SwitchonEDrawDebugTrace (Variables|HitDetection|GetDebugDrawType)
    (:None
      (Variables|HitDetection|SetDebugDrawType "ForOneFrame"))
    (:ForOneFrame
      (Variables|HitDetection|SetDebugDrawType "ForDuration"))
    (:ForDuration
      (Variables|HitDetection|SetDebugDrawType "Persistent"))
    (:Persistent
      (Variables|HitDetection|SetDebugDrawType "None")))
  (bind _asmcsgame_instance (Utilities|GetGameInstance))
  (Default|ShowClientMessage _asmcsgame_instance "SYSTEM" (Utilities|Text|FormatText "Trace Lines are set to display: {display}" (Utilities|Text|ToText(String) (Utilities|String|EnumtoString (Variables|HitDetection|GetDebugDrawType))))))

(event Custom|ToggleHitInfo
  ;[1 0.8453 0.2404] DEBUG: Toggle trace lines / hit information.
  (bind _output_get (Variables|HitDetection|SetbDisplayHitInfo (not (Variables|HitDetection|GetbDisplayHitInfo))))
  (if _output_get
    (Development|PrintString "Hit info is ON")
    (else
      (Development|PrintString "Hit info is OFF"))))

(event Custom|EnableHitDetection
  (params (Enable :type Boolean))
  ;[1 0.38 0.38] Enables/Disables Hit Detection traces for this weapon
  (bind _output_get (Variables|HitDetection|SethitDetectionEnabled Enable))
  (CallFunction|ToggleWeaponTrails _output_get)
  (if (and (Variables|HitDetection|GethitDetectionEnabled) (Variables|Weapon|GetIsWeaponDrawn?))
    (Variables|HitDetection|SetDeltaTimeInMesh 0.0)
    (Variables|HitDetection|SetDebugDrawType (Variables|HitDetection|GetDebugDrawType))
    (Utilities|ResetWeaponSockets)
    (Utilities|FlowControl|Gate true) ; enters at Open
    (else
      (Utilities|FlowControl|Gate true) ; enters at Close
    )))

(event EventTick
  (params (DeltaSeconds :type Float%20%28single-precision%29))
  ;[1 0.38 0.38] Enables/Disables Hit Detection traces for this weapon
  (Variables|Globals|SetDeltaSeconds DeltaSeconds)
  (Utilities|FlowControl|Gate true
    (:Exit
      (bind (_hitresult _weaponhit_) (Utilities|WeaponTrace "TraceTypeQuery3"))
      (Variables|HitDetection|SetWeaponHitResult _hitresult)
      (if _weaponhit_
        (if (Utilities|ClassIsChildOf (Utilities|GetClass (.HitActor (Collision|BreakHitResult (Variables|HitDetection|GetWeaponHitResult)))) "Lightsaber_C") ; Did we hit the other players weapon?
          (if (Variables|HitDetection|GetbDisplayHitInfo)
            (Development|PrintString "NOT IMPLEMENTED : PrintHitInfo()"))
          (Class|ICharacter|IBladeHitBlade(Message) (Actor|GetParentActor) (Variables|HitDetection|GetWeaponHitResult))
          (elif (Utilities|ClassIsChildOf (Utilities|GetClass (.HitActor (Collision|BreakHitResult (Variables|HitDetection|GetWeaponHitResult)))) "/Game/MCS/Blueprints/MCSCharacter.MCSCharacter_C") ; Did we hit the other player?
            (if (Variables|HitDetection|GetbDisplayHitInfo)
              (Development|PrintString "NOT IMPLEMENTED : PrintHitInfo()"))
            (Class|ICharacter|IBladeHitPlayer(Message) (Actor|GetParentActor) (Variables|HitDetection|GetWeaponHitResult) (Variables|HitDetection|GetDeltaTimeInMesh))))))))

(fn ConstructionScript
  (Variables|Materials|SetDefaultLightIntesity (Variables|/Script/Engine.LightComponentBase|GetIntensity (Variables|Default|GetBladeLight)))
  (if (Variables|Weapon|GetIsWeaponDrawn?)
    _
    (else
      (Rendering|Components|Light|SetIntensity (Variables|Default|GetBladeLight) 0.0)
      (Transformation|SetWorldScale3D (Variables|Default|GetBlade) (Math|Vector|MakeVector 1.0 1.0 0.0))
      (Rendering|SetVisibility (Variables|Default|GetHilt) false true)))
  (bind _returnvalue (Rendering|Material|CreateDynamicMaterialInstance (Variables|Default|GetBlade) 0 "/Game/MCS/Materials/Glow_MI.Glow_MI" :!class /Script/Engine.PrimitiveComponent))
  (bind _output_get (Variables|Materials|SetBladeMaterial _returnvalue))
  (Rendering|Material|SetVectorParameterValue _output_get "EmissiveColor" (Variables|Materials|GetSaberColor) :!class /Script/Engine.MaterialInstanceDynamic)
  (Rendering|Components|Light|SetLightColor (Variables|Default|GetBladeLight) (Variables|Materials|GetSaberColor) true)
  (Weapon|SetCollision false))

(fn SetCollision
  (params (Enable :type Boolean))
  (if Enable
    (Collision|SetCollisionEnabled (Variables|Default|GetHilt) "QueryAndPhysics")
    (Collision|SetCollisionEnabled (Variables|Default|GetBlade) "QueryAndPhysics")
    (else
      (Collision|SetCollisionEnabled (Variables|Default|GetHilt) "NoCollision")
      (Collision|SetCollisionEnabled (Variables|Default|GetBlade) "NoCollision"))))

(fn PrintPhysicsInfo
  (Development|PrintString (Utilities|GetDisplayName self))
  (Development|PrintString (Utilities|String|Append "Linear:  " (Utilities|String|ToString(Vector) (Variables|HitDetection|GetLinearVelocity)) "      " "Angular:  " (Utilities|String|ToString(Vector) (Variables|HitDetection|GetAngularVelocity)) "      " "Linear at Point:  " (Utilities|String|ToString(Vector) (Variables|HitDetection|GetLinearVelocityAtPoint)))))