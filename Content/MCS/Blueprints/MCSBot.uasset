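; MCSBot is an AI lightsaber combatant built on a shared character base class.
; InitSpawn starts its behavior tree, seeds blackboard defaults and plays a spawn sound.
; Multicast-named events handle attack, abort, jump and roll by driving MCSBotAnimation, with attacks toggling saber hit detection and randomizing swing direction from AttackDirection.
; Tick simulates movement input during rolls and eases aim pitch toward random targets to vary forward/back lean.
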(event Custom|BotHasSpawned
  (params (BotLocation :type Vector))
  ;[1 1 1] Play spawn sound for all the clients
  (Audio|PlaySoundatLocation "/Game/MCS/Sounds/Bot/Spawn_Cue.Spawn_Cue" BotLocation))

(event EventTick
  (params (DeltaSeconds :type Float%20%28single-precision%29))
  (|CallParentFunction DeltaSeconds)
  ;[1 1 1] Randomize the AI leaning forward/back
  (Utilities|UpdatePitch)
  ;[1 1 1] While rolling : Simulates a user pressing the movement input keys implemented in the character base class
  (if (Variables|Default|GetIsRolling?)
    (switch Utilities|FlowControl|Switch|SwitchonMCSAttackDirection (Variables|Default|GetAttackDirection)
      (:NewEnumerator0
        (CallFunction|MoveForward 1.0))
      (:NewEnumerator7
        (CallFunction|MoveForward -1.0))
      (:NewEnumerator5
        (CallFunction|MoveRight 1.0))
      (:NewEnumerator6
        (CallFunction|MoveRight -1.0)))))

(event EventInitSpawn
  (bind _asmcsbot_controller (Utilities|Casting|CastToMCSBotController (Pawn|GetController))
    (:then
      (AI|RunBehaviorTree _asmcsbot_controller "/Game/MCS/Blueprints/AI/MCSBot_BTree.MCSBot_BTree")
      (CallFunction|BotHasSpawned (Transformation|GetActorLocation))
      ;[1 1 1] Set any default blackboard values for the AI
      (AI|Components|Blackboard|SetValueasFloat (AI|GetBlackboard self) (Utilities|Name|MakeLiteralName "attackRadius") (Variables|Default|GetDefaultAttackRadius))
      (AI|Components|Blackboard|SetValueasBool (AI|GetBlackboard self) (Utilities|Name|MakeLiteralName "InCombatRange") false))
    (:CastFailed
      (Development|PrintString "Cast Failed: MCSBotController :: MCSBot EventGraph"))))

(event Custom|AI_RollMulticast
  ;[1 1 1] AI Rolling
  (if (not (Variables|Default|GetIsAttacking?))
    (Variables|Default|SetIsCrouching? true)
    (bind _asmcsbot_animation (Utilities|Casting|CastToMCSBotAnimation (Components|SkeletalMesh|GetAnimInstance (Variables|Character|GetMesh))))
    (Variables|/Game/MCS/Blueprints/MCSAnimation.MCSAnimation_C|SetIsCrouching? _asmcsbot_animation (Variables|Default|GetIsCrouching?))
    (Variables|/Game/MCS/Blueprints/MCSAnimation.MCSAnimation_C|SetAttackDirection _asmcsbot_animation (Variables|Default|GetAttackDirection))
    (Utilities|FlowControl|Delay 0.1)
    (Variables|Default|SetIsCrouching? false)
    (bind _asmcsbot_animation_2 (Utilities|Casting|CastToMCSBotAnimation (Components|SkeletalMesh|GetAnimInstance (Variables|Character|GetMesh))))
    (Variables|/Game/MCS/Blueprints/MCSAnimation.MCSAnimation_C|SetIsCrouching? _asmcsbot_animation_2 (Variables|Default|GetIsCrouching?))))

(event Custom|AI_Walk
  ;[1 1 1] AI Walk/Run
  (if (Variables|Default|GetIsSprinting?)
    (Variables|Default|SetIsSprinting? false)
    (CallFunction|OnToggleSprintMulticast)))

(event Custom|AI_AbortAttackMulticast
  ;[1 1 1] AI Attack
  (bind _asmcsbot_animation (Utilities|Casting|CastToMCSBotAnimation (Components|SkeletalMesh|GetAnimInstance (Variables|Character|GetMesh))))
  (Default|AbortAttack _asmcsbot_animation))

(event Custom|AI_AttackMulticast
  (bind _lightsabercomponent (Variables|Default|GetLightsaberComponent))
  (bind _childactor (Variables|/Script/Engine.ChildActorComponent|GetChildActor _lightsabercomponent))
  ;[1 1 1] AI Attack
  (if (and (Variables|Default|GetCanAttack?) (not (Variables|Default|GetIsRolling?)))
    (Math|Integer|IncrementInt (Variables|Default|GetComboCount)
      (:%20%20
        (Utilities|IsValid _childactor
          (:Is%20Valid
            (bind _aslightsaber (Utilities|Casting|CastToLightsaber _childactor))
            (Default|EnableHitDetection _aslightsaber true)
            (Variables|Default|SetHitCount 0)
            (Variables|Default|SetAttackTime 0.0)
            (Variables|Default|SetCanStillAttack? false)
            (Variables|Default|SetIsAttacking? true)
            (bind _direction (CallFunction|GetBotAttackDirection))
            (bind _asmcsbot_animation (Utilities|Casting|CastToMCSBotAnimation (Components|SkeletalMesh|GetAnimInstance (Variables|Character|GetMesh))))
            (Variables|/Game/MCS/Blueprints/MCSAnimation.MCSAnimation_C|SetAttackDirection _asmcsbot_animation _direction)
            (Default|OnAttack _asmcsbot_animation)))))))

(event Custom|AI_Run
  ;[1 1 1] AI Walk/Run
  (if (Variables|Default|GetIsSprinting?)
    (Variables|Default|SetIsSprinting? true)
    (CallFunction|OnToggleSprintMulticast)))

(event Custom|AI_JumpMulticast
  (params (Duration :type Float%20%28single-precision%29))
  ;[1 1 1] AI Jumping
  (Variables|Default|SetJumpDuration Duration)
  (Variables|Default|SetIsJumpPressed? true)
  (Variables|Default|SetAttackDirection (Variables|Default|GetAttackDirection))
  (Character|Jump)
  (bind _asmcsbot_animation (Utilities|Casting|CastToMCSBotAnimation (Components|SkeletalMesh|GetAnimInstance (Variables|Character|GetMesh))))
  (Variables|/Game/MCS/Blueprints/MCSAnimation.MCSAnimation_C|SetIsJumpPressed? _asmcsbot_animation (Variables|Default|GetIsJumpPressed?))
  (Variables|/Game/MCS/Blueprints/MCSAnimation.MCSAnimation_C|SetAttackDirection _asmcsbot_animation (Variables|Default|GetAttackDirection))
  (Utilities|FlowControl|Delay (Variables|Default|GetJumpDuration))
  (Character|StopJumping)
  (Variables|Default|SetJumpDuration 0.0)
  (Variables|Default|SetIsJumpPressed? false)
  (Variables|Default|SetAttackDirection (Variables|Default|GetAttackDirection))
  (bind _asmcsbot_animation_2 (Utilities|Casting|CastToMCSBotAnimation (Components|SkeletalMesh|GetAnimInstance (Variables|Character|GetMesh))))
  (Variables|/Game/MCS/Blueprints/MCSAnimation.MCSAnimation_C|SetIsJumpPressed? _asmcsbot_animation_2 (Variables|Default|GetIsJumpPressed?)))

(event EventAttackEndedMulticast
  (bind _lightsabercomponent (Variables|Default|GetLightsaberComponent))
  (bind _childactor (Variables|/Script/Engine.ChildActorComponent|GetChildActor _lightsabercomponent))
  ;[1 1 1] AI Attack
  (Variables|Default|SetIsAttacking? false)
  (Variables|Default|SetIsRecovering? false)
  (Variables|Default|SetComboCount 0)
  (Variables|Default|SetCombatStance "NewEnumerator1")
  (Variables|Default|SetAttackTime 0.0)
  (Variables|Default|SetHitCount 0)
  (Utilities|IsValid _childactor
    (:Is%20Valid
      (bind _aslightsaber (Utilities|Casting|CastToLightsaber _childactor))
      (Default|EnableHitDetection _aslightsaber false))))

(fn ConstructionScript
  (|CallParentFunction))

(fn RollRightLeft
  (params (Speed :type Float%20%28single-precision%29))
  (Transformation|SetActorLocation (+ (Transformation|GetActorLocation) (* (Transformation|GetActorRightVector) (* (Variables|Default|GetDeltaSeconds) Speed))) false false)
  (return))

(fn GetBotAttackDirection
  (switch Utilities|FlowControl|Switch|SwitchonMCSAttackDirection (Variables|Default|GetAttackDirection)
    (:NewEnumerator0
      (switch int (Math|Random|RandomIntegerinRange 0 6)
        (:0
          (Variables|Default|SetBotAttackDirection "NewEnumerator1"))
        (:1
          (Variables|Default|SetBotAttackDirection "NewEnumerator2"))
        (:2
          (Variables|Default|SetBotAttackDirection "NewEnumerator6"))
        (:3
          (Variables|Default|SetBotAttackDirection "NewEnumerator5"))
        (:4
          (Variables|Default|SetBotAttackDirection "NewEnumerator3"))
        (:5
          (Variables|Default|SetBotAttackDirection "NewEnumerator4"))
        (:6
          (Variables|Default|SetBotAttackDirection "NewEnumerator0"))))
    (:NewEnumerator5
      (switch int (Math|Random|RandomIntegerinRange 0 2)
        (:0
          (Variables|Default|SetBotAttackDirection "NewEnumerator5"))
        (:1
          (Variables|Default|SetBotAttackDirection "NewEnumerator3"))
        (:2
          (Variables|Default|SetBotAttackDirection "NewEnumerator1"))))
    (:NewEnumerator6
      (switch int (Math|Random|RandomIntegerinRange 0 2)
        (:0
          (Variables|Default|SetBotAttackDirection "NewEnumerator6"))
        (:1
          (Variables|Default|SetBotAttackDirection "NewEnumerator4"))
        (:2
          (Variables|Default|SetBotAttackDirection "NewEnumerator2")))))
  (return (Variables|Default|GetBotAttackDirection)))

(fn RollForward
  (params (Speed :type Float%20%28single-precision%29))
  (Transformation|SetActorLocation (+ (Transformation|GetActorLocation) (* (Transformation|GetActorForwardVector) (* (Variables|Default|GetDeltaSeconds) Speed))) false false)
  (return))