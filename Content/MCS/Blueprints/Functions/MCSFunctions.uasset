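; MCS function library with two stateless vector math helpers for orientation and angle queries.
; NormalToRotator derives roll from the normal's Y/Z and negated pitch from its X/Z using Atan2, leaving yaw at zero.
; AngleBetweenVectors normalizes both inputs and returns the angle between them in degrees through the arccosine of their dot product.
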(fn NormaltoRotator
  (params (Normal :type Vector))
  (bind (_x _y _z) (Math|Vector|BreakVector Normal))
  (return (Math|Rotator|MakeRotator (Math|Trig|Atan2(Radians) _y _z) (* (Math|Trig|Atan2(Radians) _x _z) -1.0) 0.0)))

(fn AngleBetweenVectors
  (params (A :type Vector) (B :type Vector))
  (return (Class|KismetMathLibrary|DegAcos (Math|Vector|DotProduct (Math|Vector|Normalize A) (Math|Vector|Normalize B)))))