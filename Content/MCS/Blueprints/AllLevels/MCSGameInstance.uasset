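; Game instance that owns the game's front-end flow: menus, loading screen, player profile and multiplayer sessions.
; The profile loads from a save slot, and a missing save or empty player name opens the options menu instead of the main menu.
; Session create, join and destroy events handle lobby hosting on SunTemple, while network and travel failures become error messages.
; Most widgets are created once and reused, with timed server, error and client popups.
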(event Custom|ShowMainMenu
  (bind _returnvalue (Game|GetPlayerController 0))
  ;[0 0.7294 1] Show main menu and enable the mouse cursor
  (Utilities|IsValid (Variables|Widgets|GetmainMenu)
    (:Is%20Valid
      _)
    (:Is%20Not%20Valid
      (bind _returnvalue_2 (UserInterface|CreateWidget "/Game/MCS/UI/MainMenu/MainMenu.MainMenu_C" _returnvalue))
      (bind _output_get (Variables|Widgets|SetmainMenu _returnvalue_2))
      (Utilities|IsValid _output_get
        (:Is%20Valid
          _))))
  (UserInterface|Viewport|AddtoViewport (Variables|Widgets|GetmainMenu) 0)
  (Variables|/Script/Engine.PlayerController|SetbShowMouseCursor _returnvalue true)
  (Input|SetInputModeUIOnly _returnvalue (Variables|Widgets|GetmainMenu) "DoNotLock")
  (CallFunction|DisplayVersion))

(event Custom|ShowServerMenu
  ;[0 0.7294 1] Show server menu (search for host servers or add IP)
  (bind _returnvalue (UserInterface|CreateWidget "/Game/MCS/UI/MainMenu/ServerMenu.ServerMenu_C" (Game|GetPlayerController 0)))
  (bind _output_get (Variables|Widgets|SetserverMenu _returnvalue))
  (Utilities|IsValid _output_get
    (:Is%20Valid
      (UserInterface|Viewport|AddtoViewport _output_get 0))))

(event Custom|ShowLoadingScreen
  ;[0 0.7294 1] Show loading screen
  (Utilities|IsValid (Variables|Widgets|GetloadingScreen)
    (:Is%20Valid
      _)
    (:Is%20Not%20Valid
      (bind _returnvalue (UserInterface|CreateWidget "/Game/MCS/UI/AllLevels/LoadingScreen.LoadingScreen_C" (Game|GetPlayerController 0)))
      (bind _output_get (Variables|Widgets|SetloadingScreen _returnvalue))
      (Utilities|IsValid _output_get
        (:Is%20Valid
          _))))
  (UserInterface|Viewport|AddtoViewport (Variables|Widgets|GetloadingScreen) 0))

(event Custom|JoinServer
  (params (SessionToJoin :type Blueprint%20Session%20Result%20Structure))
  ;[0 1 0.2708] Join server.  Called from server menu.
  (CallFunction|ShowLoadingScreen)
  (|JoinSession (Game|GetPlayerController 0) SessionToJoin
    (:OnFailure
      (Utilities|DisplayErrorMessage "FAILED TO JOIN SESSION"))))

(event Custom|ShowClientMessage
  (params (category :type Text) (clientMessage :type Text))
  ;[0 0.7294 1] Client Messages
  (Variables|Messages|SetmessageCategory category)
  (Variables|Messages|SetclientMessageText clientMessage)
  (Utilities|IsValid (Variables|Widgets|GetclientMessage)
    (:Is%20Valid
      _)
    (:Is%20Not%20Valid
      (bind _returnvalue (UserInterface|CreateWidget "/Game/MCS/UI/AllLevels/ClientMessage.ClientMessage_C" (Game|GetPlayerController 0)))
      (bind _output_get (Variables|Widgets|SetclientMessage _returnvalue))
      (Utilities|IsValid _output_get
        (:Is%20Valid
          _))))
  (Default|SetMessage (Variables|Widgets|GetclientMessage) (Variables|Messages|GetmessageCategory) (Variables|Messages|GetclientMessageText))
  (if (not (UserInterface|Viewport|IsinViewport (Variables|Widgets|GetclientMessage)))
    (UserInterface|Viewport|AddtoViewport (Variables|Widgets|GetclientMessage) 0))
  (Utilities|FlowControl|RetriggerableDelay (Variables|Messages|GetmessageDuration))
  (Widget|RemovefromParent (Variables|Widgets|GetclientMessage)))

(event Custom|ShowOptionsMenu
  ;[0 0.7294 1] Show options menu
  (Utilities|IsValid (Variables|Widgets|GetoptionsMenu)
    (:Is%20Valid
      _)
    (:Is%20Not%20Valid
      (bind _returnvalue (UserInterface|CreateWidget "/Game/MCS/UI/MainMenu/PlayerOptionsMenu.PlayerOptionsMenu_C" (Game|GetPlayerController 0)))
      (bind _output_get (Variables|Widgets|SetoptionsMenu _returnvalue))
      (Utilities|IsValid _output_get
        (:Is%20Valid
          _))))
  (UserInterface|Viewport|AddtoViewport (Variables|Widgets|GetoptionsMenu) 0))

(event Custom|ShowErrorMessage
  (params (ErrorMessage :type Text))
  ;[0 0.7294 1] Error Messages
  (Variables|Messages|SeterrorMessageText ErrorMessage)
  (Utilities|IsValid (Variables|Widgets|GeterrorMessage)
    (:Is%20Valid
      _)
    (:Is%20Not%20Valid
      (bind _returnvalue (UserInterface|CreateWidget "/Game/MCS/UI/AllLevels/ErrorMessage.ErrorMessage_C" (Game|GetPlayerController 0)))
      (bind _output_get (Variables|Widgets|SeterrorMessage _returnvalue))
      (Utilities|IsValid _output_get
        (:Is%20Valid
          _))))
  (Default|SetMessage (Variables|Widgets|GeterrorMessage) (Variables|Messages|GeterrorMessageText))
  (if (not (UserInterface|Viewport|IsinViewport (Variables|Widgets|GeterrorMessage)))
    (UserInterface|Viewport|AddtoViewport (Variables|Widgets|GeterrorMessage) 0))
  (Utilities|FlowControl|RetriggerableDelay (Variables|Messages|GetmessageDuration))
  (Widget|RemovefromParent (Variables|Widgets|GeterrorMessage)))

(event Custom|ShowInGameMenu
  (bind _returnvalue (Game|GetPlayerController 0))
  ;[0 0.7294 1] Show the in game menu
  (Utilities|IsValid (Variables|Widgets|GetinGameMenu)
    (:Is%20Valid
      _)
    (:Is%20Not%20Valid
      (bind _returnvalue_2 (UserInterface|CreateWidget "/Game/MCS/UI/MainMenu/InGameMenu.InGameMenu_C" _returnvalue))
      (Variables|Widgets|SetinGameMenu _returnvalue_2)))
  (UserInterface|Viewport|AddtoViewport (Variables|Widgets|GetinGameMenu) 0)
  (Input|SetInputModeUIOnly _returnvalue 0 "DoNotLock")
  (Variables|/Script/Engine.PlayerController|SetbShowMouseCursor _returnvalue true))

(event Custom|DestroySessionCaller
  (params (playerController :type Player%20Controller%20Object%20Reference))
  ;[0 1 0.2708] Destroy session
  (|DestroySession playerController
    (:OnFailure
      (Utilities|DisplayErrorMessage "FAILED TO DESTROY SESSION"))))

(event Custom|LaunchLobby
  (params (maxPlayers :type Integer) (enableLAN? :type Boolean) (serverName :type Name))
  ;[0 1 0.2708] Launch the map and create session
  (Variables|ServerSettings|SetmaxPlayers maxPlayers)
  (Variables|ServerSettings|SetenableLAN enableLAN?)
  (Variables|ServerSettings|SetserverName serverName)
  (CallFunction|ShowLoadingScreen)
  (|Session (Game|GetPlayerController 0) (Variables|ServerSettings|GetmaxPlayers) (Variables|ServerSettings|GetenableLAN)
    (:OnSuccess
      (Game|OpenLevel(byName) "SunTemple"))
    (:OnFailure
      (Utilities|DisplayErrorMessage "FAILED TO CREATE SESSION"))))

(event Custom|DisplayVersion
  ;[1 1 1] Display the project version number
  (Utilities|IsValid (Variables|Widgets|GetprojectVersion)
    (:Is%20Valid
      _)
    (:Is%20Not%20Valid
      (bind _returnvalue (UserInterface|CreateWidget "/Game/MCS/Blueprints/AllLevels/ProjectVersion.ProjectVersion_C" (Game|GetPlayerController 0)))
      (Variables|Widgets|SetprojectVersion _returnvalue)))
  (if (not (UserInterface|Viewport|IsinViewport (Variables|Widgets|GetprojectVersion)))
    (UserInterface|Viewport|AddtoViewport (Variables|Widgets|GetprojectVersion) 0)))

(event Custom|SavedProfileCheck
  (bind _returnvalue (Game|GetPlayerController 0))
  ;[1 1 1] Check if the players profile has already been saved and is valid
  (bind _returnvalue_2 (SaveGame|DoesSaveGameExist (Variables|PlayerProfile|GetPlayerProfileSave)))
  (if _returnvalue_2
    (PlayerProfile|LoadProfile)
    (bind _isvalid (PlayerProfile|CheckProfile))
    (bind _output_get (Variables|PlayerProfile|SetIsValidProfile? _isvalid))
    (if _output_get
      (CallFunction|ShowMainMenu)
      (else
        (CallFunction|ShowOptionsMenu :!label _label)
        (Variables|/Script/Engine.PlayerController|SetbShowMouseCursor _returnvalue true)
        (Variables|PlayerProfile|SetIsValidProfile? false)
        (Input|SetInputModeUIOnly _returnvalue (Variables|Widgets|GetmainMenu) "DoNotLock")))
    (else
      (PlayerProfile|SaveProfile)
      (goto _label))))

(event Custom|ShowServerMessage
  (params (message :type Text))
  ;[0 0.7294 1] Show server messages
  (Variables|Messages|SetserverMessageText message)
  (Utilities|IsValid (Variables|Widgets|GetserverMessage)
    (:Is%20Valid
      _)
    (:Is%20Not%20Valid
      (bind _returnvalue (UserInterface|CreateWidget "/Game/MCS/UI/AllLevels/ServerMessage.ServerMessage_C" (Game|GetPlayerController 0)))
      (bind _output_get (Variables|Widgets|SetserverMessage _returnvalue))
      (Utilities|IsValid _output_get
        (:Is%20Valid
          _))))
  (Default|SetMessage (Variables|Widgets|GetserverMessage) (Variables|Messages|GetserverMessageText))
  (if (not (UserInterface|Viewport|IsinViewport (Variables|Widgets|GetserverMessage)))
    (UserInterface|Viewport|AddtoViewport (Variables|Widgets|GetserverMessage) 0))
  (Utilities|FlowControl|RetriggerableDelay (Variables|Messages|GetmessageDuration))
  (Widget|RemovefromParent (Variables|Widgets|GetserverMessage)))

(event EventHandleNetworkError
  (params (FailureType :type ENetworkFailure%20Enum :default "NetDriverAlreadyExists") (bIsServer :type Boolean))
  (bind _outputstring (ErrorHandling|NetErrortoString FailureType))
  ;[1 0.38 0.38] Network and travel failure error handling
  (if bIsServer
    _
    (else
      _))
  (Development|PrintString _outputstring)
  (CallFunction|ShowErrorMessage (Utilities|Text|ToText(String) _outputstring)))

(event EventHandleTravelError
  (params (FailureType :type ETravelFailure%20Enum :default "NoLevel"))
  (bind _outputstring (ErrorHandling|TravelErrortoString FailureType))
  ;[1 0.38 0.38] Network and travel failure error handling
  (Development|PrintString _outputstring)
  (CallFunction|ShowErrorMessage (Utilities|Text|ToText(String) _outputstring)))

(fn NetErrortoString
  (params (failureType :type ENetworkFailure%20Enum :default "NetDriverAlreadyExists"))
  (return (Utilities|String|EnumtoString failureType)))

(fn TravelErrortoString
  (params (failureType :type ETravelFailure%20Enum :default "NoLevel"))
  (return (Utilities|String|EnumtoString failureType)))

(fn LoadProfile
  (bind _returnvalue (SaveGame|LoadGamefromSlot (Variables|PlayerProfile|GetPlayerProfileSave)))
  (bind _asmcsplayer_save_game (Utilities|Casting|CastToMCSPlayerSaveGame _returnvalue)
    (:then
      (Variables|PlayerProfile|SetplayerSaveGameRef _asmcsplayer_save_game))
    (:CastFailed
      (CallFunction|ShowErrorMessage "Failed to load player profile"))))

(fn SaveProfile
  (Utilities|IsValid (Variables|PlayerProfile|GetplayerSaveGameRef)
    (:Is%20Valid
      _)
    (:Is%20Not%20Valid
      (bind _returnvalue (SaveGame|CreateSaveGameObject "/Game/MCS/Blueprints/AllLevels/MCSPlayerSaveGame.MCSPlayerSaveGame_C"))
      (Variables|PlayerProfile|SetplayerSaveGameRef _returnvalue)))
  (bind _returnvalue_2 (SaveGame|SaveGametoSlot (Variables|PlayerProfile|GetplayerSaveGameRef) (Variables|PlayerProfile|GetPlayerProfileSave)))
  (return _returnvalue_2))

(fn GetPlayerProfile
  (bind _playersavegameref (Variables|PlayerProfile|GetplayerSaveGameRef))
  (Utilities|IsValid _playersavegameref
    (:Is%20Valid
      (return (Variables|/Game/MCS/Blueprints/AllLevels/MCSPlayerSaveGame.MCSPlayerSaveGame_C|GetPlayerProfile _playersavegameref)))
    (:Is%20Not%20Valid
      (CallFunction|ShowErrorMessage "Unable to get player profile"))))

(fn CheckProfile
  (Utilities|IsValid (Variables|PlayerProfile|GetplayerSaveGameRef)
    (:Is%20Valid
      (return (not (Utilities|Text|TextIsEmpty (.PlayerName (Utilities|Struct|BreakMCSPlayerInfo (Variables|/Game/MCS/Blueprints/AllLevels/MCSPlayerSaveGame.MCSPlayerSaveGame_C|GetPlayerProfile (Variables|PlayerProfile|GetplayerSaveGameRef))))))))
    (:Is%20Not%20Valid
      (return false))))