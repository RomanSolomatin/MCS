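; MCSSpectatorPawn is the pawn for spectating players, giving an overhead view of the combat characters.
; On BeginPlay, if LookAtPlayer is set, it moves above and beside the first MCSCharacter found, despite a comment saying random, and aims the control rotation at it once.
; It then shows the "Spectating" role on player 0's MCSPlayerHUD.
; Escape opens the in-game menu through MCSGameInstance.
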(event EventBeginPlay
  (bind _returnvalue (Pawn|GetController))
  ;[1 1 1] Spawn above combat players then rotate to look at a random player
  (if (Variables|Default|GetbLookAtPlayer)
    (bind _outactors (Actor|GetAllActorsOfClass "/Game/MCS/Blueprints/MCSCharacter.MCSCharacter_C"))
    (Utilities|IsValid (Utilities|Array|Get(acopy) _outactors)
      (:Is%20Valid
        (Utilities|IsValid _returnvalue
          (:Is%20Valid
            (Transformation|SetActorLocation (Math|Vector|MakeVector (+ (.X (Math|Vector|BreakVector (Transformation|GetActorLocation (Utilities|Array|Get(acopy) _outactors)))) 3e+02) (- (.Y (Math|Vector|BreakVector (Transformation|GetActorLocation (Utilities|Array|Get(acopy) _outactors)))) 4e+02) 1.2e+03) false false)
            (Pawn|SetControlRotation _returnvalue (Math|Rotator|FindLookatRotation (Transformation|GetActorLocation) (Transformation|GetActorLocation (Utilities|Array|Get(acopy) _outactors))))
            ;[1 1 1] Show that this player is "spectating" on the HUD
            (bind _asmcsplayer_hud (Utilities|Casting|CastToMCSPlayerHUD (HUD|GetHUD (Game|GetPlayerController 0)))
              (:then
                (Default|ShowCurrentRole _asmcsplayer_hud "Spectating"))
              (:CastFailed
                (Development|PrintString "Could not cast to \"MCSPlayerHUD\"")))))))))

(event Input|KeyboardEvents|Escape
  (params (Key :type Key%20Structure))
  ;[1 1 1] Show the in game menu
  (:Pressed
    (bind _asmcsgame_instance (Utilities|Casting|CastToMCSGameInstance (Game|GetGameInstance))
      (:then
        (Default|ShowinGameMenu _asmcsgame_instance))
      (:CastFailed
        (Development|PrintString "Unable to cast to MCSGameInstance")))))

(fn ConstructionScript)