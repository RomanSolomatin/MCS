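; Player controller for MCS that links the local player's menus, chat, player list and profile to the server.
; Key inputs drive the game instance (in-game menu) and HUD (chat, player list, debug server variables).
; Profile, chat and player list requests go to the game mode, with replies shown through the HUD.
; Incoming chat plays a sound unless history is hidden, and the player's own message reopens it.
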(event Custom|DisplayChatMessage
  (params (senderName :type Text) (senderColor :type Slate%20Color%20Structure) (chatMessage :type Text))
  ;[1 1 1] Display incoming chat message
  (Variables|UI|SetSenderName senderName)
  (bind _asmcsplayer_hud (Utilities|Casting|CastToMCSPlayerHUD (HUD|GetHUD)))
  (Default|AddChatMessage (Variables|/Game/MCS/Blueprints/HUD/MCSPlayerHUD.MCSPlayerHUD_C|GetHUDWidget _asmcsplayer_hud) (Variables|UI|GetSenderName) senderColor chatMessage)
  (bind _asmcsplayer_hud_2 (Utilities|Casting|CastToMCSPlayerHUD (HUD|GetHUD)))
  (Default|FocusChatMessageInput _asmcsplayer_hud_2)
  (if (not (Variables|UI|GetChatHiddenByUser))
    (Audio|PlaySound2D "/Game/MCS/Sounds/UI/commlink_on.commlink_on" :!label _label)
    (elif (Utilities|Enum|Equal(Enum) (Variables|UI|GetSenderName) (.PlayerName (Utilities|Struct|BreakMCSPlayerInfo (Variables|PlayerProfile|GetPlayerProfile))))
      (CallFunction|ShowMessageHistory)
      (goto _label))))

(event Custom|ReceivePlayerListFromServer
  (params (PlayerList :type Array%20of%20Strings))
  ;[1 1 1] Request/receive player list from server
  (Variables|Default|SetPlayerList PlayerList)
  (bind _asmcsplayer_hud (Utilities|Casting|CastToMCSPlayerHUD (HUD|GetHUD)))
  (Default|UpdatePlayerList _asmcsplayer_hud))

(event Custom|SRV_RequestPlayerList
  ;[1 1 1] Request/receive player list from server
  (bind _asmcsgame_mode_duel (Utilities|Casting|CastToMCSGameModeDuel (Game|GetGameMode)))
  (Default|RequestPlayerList _asmcsgame_mode_duel self))

(event Custom|RequestPlayerProfile
  ;[1 1 1] Player profile has been requested by the server
  (bind _playerprofile (Class|IPlayerProfile|IGetPlayerProfile(Message) (Game|GetGameInstance)))
  (bind _output_get (Variables|PlayerProfile|SetPlayerProfile _playerprofile))
  (Variables|PlayerProfile|SetplayerUIName (.PlayerName (Utilities|Struct|BreakMCSPlayerInfo _output_get)))
  (Variables|PlayerProfile|SetplayerUIColorSlate (Utilities|Struct|MakeSlateColor (Utilities|Struct|MakeLinearColor (.R (Utilities|Struct|BreakLinearColor (.SaberColor (Utilities|Struct|BreakMCSPlayerInfo _output_get)))) (.G (Utilities|Struct|BreakLinearColor (.SaberColor (Utilities|Struct|BreakMCSPlayerInfo _output_get)))) (.B (Utilities|Struct|BreakLinearColor (.SaberColor (Utilities|Struct|BreakMCSPlayerInfo _output_get)))) 1.0)))
  (CallFunction|SendPlayerProfile self (Variables|PlayerProfile|GetPlayerProfile)))

(event Custom|SendPlayerProfile
  (params (controller :type MCS%20Player%20Controller%20Object%20Reference) (profile :type MCS%20Player%20Info%20Structure))
  ;[1 1 1] Player profile has been requested by the server
  (bind _result (Class|IGameMode|IUpdatePlayerProfile(Message) (Game|GetGameMode) controller profile))
  (if (not _result)
    (Development|PrintString "INVALID PROFILE")))

(event Custom|DisplayServerMessage
  (params (message :type Text))
  ;[1 1 1] Display messages sent from the server
  (Networking|SwitchHasAuthority
    (:Remote
      (bind _asmcsgame_instance (Utilities|Casting|CastToMCSGameInstance (Game|GetGameInstance)))
      (Default|ShowServerMessage _asmcsgame_instance message))))

(event Custom|SendChatMessageToServer
  (params (playerName :type Text) (playerColor :type Slate%20Color%20Structure) (playerChatMessage :type Text))
  ;[1 1 1] Broadcast chat message
  (Class|IChat|SendChatMessage(Message) (Game|GetGameMode) playerName playerColor playerChatMessage))

(event EventBeginPlay
  (if (Pawn|IsLocalController)
    (bind _asmcsgame_instance (Utilities|Casting|CastToMCSGameInstance (Game|GetGameInstance)))
    (bind _output_get (Variables|Default|SetGameInstanceRef _asmcsgame_instance))
    (Default|CheckProfileExists _output_get)
    (Default|DisplayVersion (Variables|Default|GetGameInstanceRef))
    (bind _asmcsplayer_hud (Utilities|Casting|CastToMCSPlayerHUD (HUD|GetHUD))
      (:then
        (Default|HideCurrentRole _asmcsplayer_hud))
      (:CastFailed
        (Development|PrintString "Could not cast to \"MCSPlayerHUD\"")))))

(event EventTick
  (params (DeltaSeconds :type Float%20%28single-precision%29)))

(event Input|ActionEvents|InputActionPlayerList
  (params (Key :type Key%20Structure))
  ;[1 1 1] Request/receive player list from server
  (:Pressed
    (bind _asmcsplayer_hud (Utilities|Casting|CastToMCSPlayerHUD (HUD|GetHUD)))
    (Default|TogglePlayerList _asmcsplayer_hud)
    (CallFunction|SRVRequestPlayerList)))

(event Input|KeyboardEvents|T
  (params (Key :type Key%20Structure))
  ;[1 1 1] Show the chat interface
  (:Pressed
    (bind _asmcsplayer_hud (Utilities|Casting|CastToMCSPlayerHUD (HUD|GetHUD)))
    (Default|ShowChatMessageInput _asmcsplayer_hud)))

(event Input|KeyboardEvents|AltT
  (params (Key :type Key%20Structure))
  ;[1 1 1] Toggle chat message history
  (:Pressed
    (if (Variables|UI|GetChatHiddenByUser)
      (CallFunction|ShowMessageHistory)
      (else
        (CallFunction|HideMessageHistory)))))

(event Input|KeyboardEvents|F2
  (params (Key :type Key%20Structure))
  ;[1 1 1] Show/Hide server variables window for play testing purposes
  (:Pressed
    (bind _asmcsplayer_hud (Utilities|Casting|CastToMCSPlayerHUD (HUD|GetHUD)))
    (Default|ShowServerVariables _asmcsplayer_hud)))

(event Input|KeyboardEvents|Escape
  (params (Key :type Key%20Structure))
  ;[0 0.7294 1] Show the in game menu
  (:Pressed
    (bind _asmcsgame_instance (Utilities|Casting|CastToMCSGameInstance (Game|GetGameInstance)))
    (Default|ShowinGameMenu _asmcsgame_instance)))

(fn ConstructionScript
  (if (Pawn|IsLocalController)
    _))

(fn ShowMessageHistory
  (bind _asmcsplayer_hud (Utilities|Casting|CastToMCSPlayerHUD (HUD|GetHUD)))
  (Default|ShowChatWindow _asmcsplayer_hud)
  (Variables|UI|SetChatHiddenByUser false))

(fn HideMessageHistory
  (bind _asmcsplayer_hud (Utilities|Casting|CastToMCSPlayerHUD (HUD|GetHUD)))
  (Default|HideChatWindow _asmcsplayer_hud)
  (Variables|UI|SetChatHiddenByUser true))