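; Player HUD Blueprint for MCS that creates the main HUD widget on BeginPlay and exposes events to show and hide its elements.
; It controls the role text, chat window and chat input, switching cursor and input mode for typing.
; The player list widget is created lazily, fed from MCSPlayerController and toggled by FlipFlop.
; Server page and server variable events are empty stubs, with their former logic left disconnected.
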(event Custom|ShowChatMessageInput
  (bind _hudwidget (Variables|Widgets|GetHUDWidget))
  (bind _hudwidget_2 (Variables|Widgets|GetHUDWidget))
  (bind _chatmessageinput (Variables|/Game/MCS/Blueprints/HUD/MCSPlayerHUDWidget.MCSPlayerHUDWidget_C|GetChatMessageInput _hudwidget))
  (bind _chatmessageinput_2 (Variables|/Game/MCS/Blueprints/HUD/MCSPlayerHUDWidget.MCSPlayerHUDWidget_C|GetChatMessageInput _hudwidget_2))
  ;[1 1 1] User Chat message
  (Default|Init _chatmessageinput)
  (if (not (UserInterface|Viewport|IsinViewport _chatmessageinput))
    (UserInterface|Viewport|AddtoViewport (Variables|/Game/MCS/Blueprints/HUD/MCSPlayerHUDWidget.MCSPlayerHUDWidget_C|GetChatMessageInput (Variables|Widgets|GetHUDWidget)) 0))
  (Variables|/Script/Engine.PlayerController|SetbShowMouseCursor (Game|GetPlayerController 0) true)
  (Widget|SetVisibility _chatmessageinput_2 "Visible")
  (Input|SetInputModeUIOnly (Game|GetPlayerController 0) 0 "DoNotLock")
  (Widget|SetKeyboardFocus (Variables|/Game/MCS/UI/AllLevels/ChatMessage.ChatMessage_C|GettbChatMessageText _chatmessageinput_2)))

(event Custom|TogglePlayerList
  (Utilities|FlowControl|FlipFlop
    (:A
      (CallFunction|ShowPlayerList))
    (:B
      (CallFunction|HidePlayerList))))

(event Custom|ShowChatWindow
  ;[1 1 1] Chat window
  (Default|ShowChatWindow (Variables|Widgets|GetHUDWidget)))

(event Custom|ShowCurrentRole
  (params (CurrentRoleText :type Text))
  (bind _hudwidget (Variables|Widgets|GetHUDWidget))
  (bind _tbcurrentrole (Variables|/Game/MCS/Blueprints/HUD/MCSPlayerHUDWidget.MCSPlayerHUDWidget_C|GettbCurrentRole _hudwidget))
  ;[1 1 1] Current player role text (spectator, etc.)
  (Utilities|IsValid (Variables|Widgets|GetHUDWidget)
    (:Is%20Valid
      (Rendering|Components|TextRender|SetText _tbcurrentrole CurrentRoleText)
      (Widget|SetVisibility _tbcurrentrole "Visible"))))

(event Custom|HideCurrentRole
  ;[1 1 1] Current player role text (spectator, etc.)
  (Widget|SetVisibility (Variables|/Game/MCS/Blueprints/HUD/MCSPlayerHUDWidget.MCSPlayerHUDWidget_C|GettbCurrentRole (Variables|Widgets|GetHUDWidget)) "Hidden"))

(event Custom|FocusChatMessageInput
  ;[1 1 1] User Chat message
  (Widget|SetKeyboardFocus (Variables|/Game/MCS/UI/AllLevels/ChatMessage.ChatMessage_C|GettbChatMessageText (Variables|/Game/MCS/Blueprints/HUD/MCSPlayerHUDWidget.MCSPlayerHUDWidget_C|GetChatMessageInput (Variables|Widgets|GetHUDWidget)))))

(event Custom|ShowServerPage)

(event Custom|ToggleChatWindow
  ;[1 1 1] Chat window
  (if (Widget|IsVisible (Variables|/Game/MCS/Blueprints/HUD/MCSPlayerHUDWidget.MCSPlayerHUDWidget_C|GetChatWindow (Variables|Widgets|GetHUDWidget)))
    (CallFunction|HideChatWindow)
    (else
      (CallFunction|ShowChatWindow))))

(event Custom|ShowServerVariables)

(event Custom|ToggleServerPage)

(event Custom|HideServerVariables)

(event Custom|ShowPlayerList
  (Utilities|IsValid (Variables|Widgets|GetPlayerList)
    (:Is%20Valid
      _)
    (:Is%20Not%20Valid
      (bind _returnvalue (UserInterface|CreateWidget "/Game/MCS/Blueprints/HUD/MCSGenericList.MCSGenericList_C" (Game|GetPlayerController 0)))
      (Variables|Widgets|SetPlayerList _returnvalue)))
  (bind _asmcsplayer_controller (Utilities|Casting|CastToMCSPlayerController (Game|GetPlayerController 0)))
  (Default|AddList (Variables|Widgets|GetPlayerList) (Variables|/Game/MCS/Blueprints/MCSPlayerController.MCSPlayerController_C|GetPlayerList _asmcsplayer_controller))
  (if (not (UserInterface|Viewport|IsinViewport (Variables|Widgets|GetPlayerList)))
    (UserInterface|Viewport|AddtoViewport (Variables|Widgets|GetPlayerList) 0)
    (elif (not (Widget|IsVisible (Variables|Widgets|GetPlayerList)))
      (Widget|SetVisibility (Variables|Widgets|GetPlayerList) "Visible"))))

(event Custom|ToggleServerVariables)

(event Custom|HideChatMessageInput
  (bind _returnvalue (Game|GetPlayerController 0))
  ;[1 1 1] User Chat message
  (Widget|SetVisibility (Variables|/Game/MCS/Blueprints/HUD/MCSPlayerHUDWidget.MCSPlayerHUDWidget_C|GetChatMessageInput (Variables|Widgets|GetHUDWidget)) "Hidden")
  (Input|SetInputModeGameOnly _returnvalue)
  (Variables|/Script/Engine.PlayerController|SetbShowMouseCursor _returnvalue false))

(event Custom|HideServerPage)

(event Custom|HidePlayerList
  (Utilities|IsValid (Variables|Widgets|GetPlayerList)
    (:Is%20Valid
      (if (Widget|IsVisible (Variables|Widgets|GetPlayerList))
        (Widget|SetVisibility (Variables|Widgets|GetPlayerList) "Hidden")))))

(event Custom|HideChatWindow
  ;[1 1 1] Chat window
  (Default|HideChatWindow (Variables|Widgets|GetHUDWidget)))

(event EventBeginPlay
  (bind _returnvalue (UserInterface|CreateWidget "/Game/MCS/Blueprints/HUD/MCSPlayerHUDWidget.MCSPlayerHUDWidget_C" (Game|GetPlayerController 0)))
  (bind _output_get (Variables|Widgets|SetHUDWidget _returnvalue))
  (UserInterface|Viewport|AddtoViewport _output_get 0)
  (CallFunction|ToggleServerPage))

(fn ConstructionScript)