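; Behavior tree task that moves an AI bot toward its current enemy until it reaches combat range.
; It writes the enemy location to the blackboard, enters combat mode at once if already near, and starts AIMoveTo.
; The task finishes as soon as the move is issued, jumping into combat mode when near the jump radius.
; Move success sets the in-combat-range key and calls FinishExecute as failed.
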(event EventReceiveExecuteAI
  (params (OwnerController :type AI%20Controller%20Object%20Reference) (ControlledPawn :type Pawn%20Object%20Reference))
  (|CallParentFunction OwnerController ControlledPawn)
  (Utilities|IsValid (Variables|Default|GetCurrentEnemy)
    (:Is%20Valid
      (if (not (Variables|/Game/MCS/Blueprints/MCSCharacter.MCSCharacter_C|GetIsDead? (Variables|Default|GetAIPawn)))
        (Class|BTFunctionLibrary|SetBlackboardValueasFloat (Variables|Blackboard|GetDistanceToEnemyKey) 0.0)
        (bind _output_get (Variables|Default|SetClosestEnemyLocation (Transformation|GetActorLocation (Variables|Default|GetCurrentEnemy))))
        (AI|BehaviorTree|SetBlackboardValueasVector (Variables|Blackboard|GetClosestEnemyLocationKey) _output_get)
        ;[1 1 1] If bot has spawned near the player - go into combat mode immediately
        (if (<= (Variables|Default|GetClosestEnemyDistance) (+ (Variables|Default|GetCombatRadius) 5e+02))
          (if (not (Variables|/Game/MCS/Blueprints/MCSCharacter.MCSCharacter_C|GetInCombatMode (Variables|Default|GetAIPawn)))
            (CallFunction|EnterCombatMode)))
        ;[1 1 1] Move into combat range
        (Variables|/Game/MCS/Blueprints/MCSCharacter.MCSCharacter_C|SetAttackDirection (Variables|Default|GetAIPawn) "NewEnumerator0")
        (AI|AIMoveTo (Variables|Default|GetAIPawn) "0, 0, 0" (Variables|Default|GetCurrentEnemy) (- (Variables|Default|GetCombatRadius) (Variables|Default|GetBufferRadius)) false
          (:then
            ;[1 1 1] Keep chasing the player until bot is in combat range
            (if (Math|Float|NearlyEqual(Float) (Variables|Default|GetClosestEnemyDistance) (Variables|Default|GetJumpRadius) 1e+01)
              (CallFunction|Jump 0.0)
              (CallFunction|EnterCombatMode)
              (elif (>= (Variables|Default|GetClosestEnemyDistance) (+ (Variables|Default|GetJumpRadius) 5e+02))
                _
                (else
                  _)))
            (AI|BehaviorTree|FinishExecute true))
          (:OnSuccess
            ;[1 1 1] We are in combat range
            (if (not (Variables|/Game/MCS/Blueprints/MCSCharacter.MCSCharacter_C|GetInCombatMode (Variables|Default|GetAIPawn)))
              (CallFunction|EnterCombatMode))
            (Class|BTFunctionLibrary|SetBlackboardValueasBool (Variables|Blackboard|GetInCombatRangeKey) true)
            (AI|BehaviorTree|FinishExecute false)))))))

(fn EnterCombatMode
  (if (not (Variables|/Game/MCS/Blueprints/MCSCharacter.MCSCharacter_C|GetInCombatMode (Variables|Default|GetAIPawn)))
    (Variables|/Game/MCS/Blueprints/MCSCharacter.MCSCharacter_C|SetInCombatMode (Variables|Default|GetAIPawn) true)))

(fn ExitCombatMode
  (if (Variables|/Game/MCS/Blueprints/MCSCharacter.MCSCharacter_C|GetInCombatMode (Variables|Default|GetAIPawn))
    (Variables|/Game/MCS/Blueprints/MCSCharacter.MCSCharacter_C|SetInCombatMode (Variables|Default|GetAIPawn) false)))