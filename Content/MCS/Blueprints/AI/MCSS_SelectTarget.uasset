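; Behavior tree service for MCS AI characters that feeds the enemy player target and AI state to the blackboard.
; Activation sets the default state; each tick reads the character's EnemyPlayerRef, using controller and pawn references cached on first tick.
; A living target is written as the follow target, with state chosen by distance against combat radius plus buffer.
; A missing or dead target restores the default state and clears the key.
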(event EventReceiveActivationAI
  (params (OwnerController :type AI%20Controller%20Object%20Reference) (ControlledPawn :type Pawn%20Object%20Reference))
  (bind _output_get (Variables|AI|SetAIState "NewEnumerator0"))
  (Class|BTFunctionLibrary|SetBlackboardValueasEnum (Variables|Keys|GetAIStateKey) _output_get))

(event EventReceiveTickAI
  (params (OwnerController :type AI%20Controller%20Object%20Reference) (ControlledPawn :type Pawn%20Object%20Reference) (DeltaSeconds :type Float%20%28single-precision%29))
  (Variables|Globals|SetDeltaSeconds DeltaSeconds)
  (if (!= (Variables|References|GetAIControllerRef) 0)
    _
    (else
      (bind _asmcsaicontroller (Utilities|Casting|CastToMCSAIController OwnerController))
      (Variables|References|SetAIControllerRef _asmcsaicontroller)
      (bind _asmcscharacter (Utilities|Casting|CastToMCSCharacter ControlledPawn))
      (Variables|References|SetAICharacterRef _asmcscharacter)))
  (Utilities|IsValid (Variables|/Game/MCS/Characters/MCSCharacter.MCSCharacter_C|GetEnemyPlayerRef (Variables|References|GetAICharacterRef))
    (:Is%20Valid
      (bind _output_get (Variables|References|SetTargetRef (Variables|/Game/MCS/Characters/MCSCharacter.MCSCharacter_C|GetEnemyPlayerRef (Variables|References|GetAICharacterRef))))
      (Utilities|IsValid _output_get
        (:Is%20Valid
          (if (not (Variables|/Game/MCS/Characters/MCSCharacter.MCSCharacter_C|GetIsDead? (Variables|References|GetTargetRef)))
            (Class|BTFunctionLibrary|SetBlackboardValueasObject (Variables|Keys|GetTargetToFollowKey) (Variables|References|GetTargetRef))
            (if (> (Math|Vector|VectorLength (- (Transformation|GetActorLocation (Variables|References|GetTargetRef)) (Transformation|GetActorLocation (Variables|References|GetAICharacterRef)))) (+ (Variables|/Game/MCS/Characters/MCSCharacter.MCSCharacter_C|GetDefaultCombatRadius (Variables|References|GetAICharacterRef)) (Variables|/Game/MCS/Characters/MCSCharacter.MCSCharacter_C|GetCombatRadiusBuffer (Variables|References|GetAICharacterRef))))
              (bind _output_get_2 (Variables|AI|SetAIState "NewEnumerator1"))
              (Class|BTFunctionLibrary|SetBlackboardValueasEnum (Variables|Keys|GetAIStateKey) _output_get_2)
              (else
                (bind _output_get_3 (Variables|AI|SetAIState "NewEnumerator5"))
                (Class|BTFunctionLibrary|SetBlackboardValueasEnum (Variables|Keys|GetAIStateKey) _output_get_3)))
            (else
              (bind _output_get_4 (Variables|AI|SetAIState "NewEnumerator0" :!label _label))
              (Class|BTFunctionLibrary|SetBlackboardValueasEnum (Variables|Keys|GetAIStateKey) _output_get_4)
              (Class|BTFunctionLibrary|SetBlackboardValueasObject (Variables|Keys|GetTargetToFollowKey)))))
        (:Is%20Not%20Valid
          (goto _label))))
    (:Is%20Not%20Valid
      (goto _label))))