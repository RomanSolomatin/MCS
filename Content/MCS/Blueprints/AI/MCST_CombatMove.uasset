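; MCST_CombatMove is an AI behavior tree task that sidesteps the character during combat.
; Each AI tick issues an AIMoveTo to the stored goal, first picking a new point 100 units randomly left or right once the last was reached.
; The task finishes as failed immediately after issuing the move.
; Move success or failure both mark the destination reached and finish as successful.
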(event EventReceiveTickAI
  (params (OwnerController :type AI%20Controller%20Object%20Reference) (ControlledPawn :type Pawn%20Object%20Reference) (DeltaSeconds :type Float%20%28single-precision%29))
  (|CallParentFunction OwnerController ControlledPawn DeltaSeconds)
  (if (not (Variables|Default|GetHasReachedDestination))
    _
    (else
      (CallFunction|ChooseNewDestination)))
  (AI|AIMoveTo (Variables|Default|GetAICharacterRef) (Variables|Default|GetGoalDestination) 0 5.0 false
    (:then
      (Variables|Default|SetHasReachedDestination false)
      (AI|BehaviorTree|FinishExecute false))
    (:OnSuccess
      (Variables|Default|SetHasReachedDestination true :!label _label)
      (AI|BehaviorTree|FinishExecute true))
    (:OnFail
      (goto _label))))

(fn ChooseNewDestination
  (bind _aicharacterref (Variables|Default|GetAICharacterRef))
  (bind _aicharacterref_2 (Variables|Default|GetAICharacterRef))
  (switch int (Math|Random|RandomIntegerinRange 0 1)
    (:0
      (Variables|Default|SetGoalDestination (+ (* (Transformation|GetActorRightVector _aicharacterref) 1e+02) (Transformation|GetWorldLocation (Variables|/Script/Engine.Character|GetMesh _aicharacterref)))))
    (:1
      (Variables|Default|SetGoalDestination (+ (* (Transformation|GetActorRightVector _aicharacterref_2) -1e+02) (Transformation|GetWorldLocation (Variables|/Script/Engine.Character|GetMesh _aicharacterref_2)))))))