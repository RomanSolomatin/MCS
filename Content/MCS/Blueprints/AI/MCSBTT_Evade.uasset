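; Behavior tree task that makes an AI character evade.
; On execute it runs the parent logic, rolls on a one-in-five random pick or otherwise jumps, then immediately finishes as failed.
; A separate EvadeMovement function, not called in this graph, picks a strafe side from the current enemy's attack direction, going left for right-side, forward or no attack and right for left-side or back attacks.
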(event EventReceiveExecuteAI
  (params (OwnerController :type AI%20Controller%20Object%20Reference) (ControlledPawn :type Pawn%20Object%20Reference))
  (|CallParentFunction OwnerController ControlledPawn)
  (switch int (Math|Random|RandomIntegerinRange 0 4)
    (:Default
      (CallFunction|Jump 0.35))
    (:0
      (CallFunction|Roll)))
  (AI|BehaviorTree|FinishExecute false))

(fn EvadeMovement
  (Utilities|IsValid (Variables|Default|GetCurrentEnemy)
    (:Is%20Valid
      (switch Utilities|FlowControl|Switch|SwitchonMCSAttackDirection (Variables|/Game/MCS/Blueprints/MCSCharacter.MCSCharacter_C|GetAttackDirection (Variables|Default|GetCurrentEnemy))
        (:NewEnumerator8
          (CallFunction|StrafeLeft false :!label _label))
        (:NewEnumerator0
          (goto _label))
        (:NewEnumerator1
          (goto _label))
        (:NewEnumerator2
          (CallFunction|StrafeRight false :!label _label_2))
        (:NewEnumerator7
          (goto _label_2))
        (:NewEnumerator3
          (goto _label))
        (:NewEnumerator4
          (goto _label_2))
        (:NewEnumerator5
          (goto _label))
        (:NewEnumerator6
          (goto _label_2))))))