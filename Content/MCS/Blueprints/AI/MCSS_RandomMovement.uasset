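; Behavior tree service that makes an MCS character strafe randomly left or right while focused on its target.
; On activation it sets the controller's focus to the blackboard target actor.
; Each tick it picks a point 500 units to either side along the pawn's right vector.
; It issues an AI move to that point unless the pause-movement blackboard flag is set.
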(event EventReceiveActivationAI
  (params (OwnerController :type AI%20Controller%20Object%20Reference) (ControlledPawn :type Pawn%20Object%20Reference))
  (AI|SetFocus OwnerController (AI|BehaviorTree|GetBlackboardValueasActor (Variables|Keys|GetTargetKey))))

(event EventReceiveTickAI
  (params (OwnerController :type AI%20Controller%20Object%20Reference) (ControlledPawn :type Pawn%20Object%20Reference) (DeltaSeconds :type Float%20%28single-precision%29))
  (Variables|Globals|SetDeltaTime DeltaSeconds)
  (bind _asmcscharacter (Utilities|Casting|CastToMCSCharacter ControlledPawn))
  (Variables|References|SetAICharacterRef _asmcscharacter)
  (switch int (Math|Random|RandomIntegerinRange 0 1)
    (:0
      (Variables|AI|SetDestination (+ (* (Transformation|GetActorRightVector (Variables|References|GetAICharacterRef)) 5e+02) (Transformation|GetActorLocation (Variables|References|GetAICharacterRef)))))
    (:1
      (Variables|AI|SetDestination (+ (* (Transformation|GetActorRightVector (Variables|References|GetAICharacterRef)) -5e+02) (Transformation|GetActorLocation (Variables|References|GetAICharacterRef))))))
  (if (not (Class|BTFunctionLibrary|GetBlackboardValueasBool (Variables|Keys|GetPauseMovementKey)))
    (AI|AIMoveTo (Variables|References|GetAICharacterRef) (Variables|AI|GetDestination) 0 5.0 false)))