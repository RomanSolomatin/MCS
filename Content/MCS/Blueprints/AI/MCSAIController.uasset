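; AI controller for MCS melee combat characters, driving movement and directional attacks.
; When the server is ready, it puts the possessed character into combat mode and starts its behavior tree.
; AI_ events feed strafing, advancing and attacks into the character's input functions, with random attacks side-weighted and throttled by a resettable DoOnce.
; AI_RandomJump is a stub, and SetMovement applies only forward input and speed because MoveRight is disconnected.
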(event Custom|AI_RandomAttack
  (Utilities|FlowControl|DoOnce false
    (:Completed
      (Combat|SetRandomAttackDirection)
      (Default|AttackPressed (Variables|References|GetCharacterRef) false)
      (Utilities|FlowControl|Delay 1.0)
      (CallFunction|ResetAttack))))

(event Custom|AI_MoveForward
  (bind _characterref (Variables|References|GetCharacterRef))
  ;[1 1 1] Movement
  (Default|CLIENTSmoothSpeed _characterref (Variables|/Game/MCS/Blueprints/MCSCharacter.MCSCharacter_C|GetDefaultCombatSpeed _characterref) 15.0)
  (Variables|/Game/MCS/Blueprints/MCSCharacter.MCSCharacter_C|SetAttackDirection (Variables|References|GetCharacterRef) "NewEnumerator0")
  (Default|MoveForward (Variables|References|GetCharacterRef) 1.0)
  (Default|MoveRight (Variables|References|GetCharacterRef) 0.0))

(event Custom|AI_StrafeRandom
  (bind _returnvalue (Pawn|GetControlRotation :!class /Script/Engine.Controller))
  (bind _characterref (Variables|References|GetCharacterRef))
  (bind _characterref_2 (Variables|References|GetCharacterRef))
  (bind _returnvalue_2 (Math|Vector|GetRightVector _returnvalue))
  ;[1 1 1] Movement
  (switch int (Math|Random|RandomIntegerinRange 0 1)
    (:0
      (Default|CLIENTSmoothSpeed _characterref_2 (Variables|/Game/MCS/Blueprints/MCSCharacter.MCSCharacter_C|GetDefaultCombatSpeed _characterref_2) 15.0)
      (Variables|/Game/MCS/Blueprints/MCSCharacter.MCSCharacter_C|SetAttackDirection (Variables|References|GetCharacterRef) "NewEnumerator5")
      (Pawn|Input|AddMovementInput (Variables|References|GetCharacterRef) _returnvalue_2 1.0 false))
    (:1
      (Default|CLIENTSmoothSpeed _characterref (Variables|/Game/MCS/Blueprints/MCSCharacter.MCSCharacter_C|GetDefaultCombatSpeed _characterref) 15.0)
      (Variables|/Game/MCS/Blueprints/MCSCharacter.MCSCharacter_C|SetAttackDirection (Variables|References|GetCharacterRef) "NewEnumerator6")
      (Pawn|Input|AddMovementInput (Variables|References|GetCharacterRef) (* _returnvalue_2 -1.0) 1.0 false))))

(event Custom|ResetAttack
  (Utilities|FlowControl|DoOnce false) ; enters at Reset
)

(event Custom|AI_RandomJump
  (params (LaunchVector :type Vector))
  (if (not (AI|Components|NavMovement|IsFalling (Variables|/Script/Engine.Character|GetCharacterMovement (Variables|References|GetCharacterRef))))
    _))

(event Custom|AI_DirectionalAttack
  (params (Direction :type MCSAttackDirection%20Enum :default "NewEnumerator8") (ComboCount :type Integer))
  (Variables|/Game/MCS/Blueprints/MCSCharacter.MCSCharacter_C|SetAttackDirection (Variables|References|GetCharacterRef) Direction)
  (Default|AttackPressed (Variables|References|GetCharacterRef) false)
  (if (== ComboCount 0)
    (Default|AttackReleased (Variables|References|GetCharacterRef))))

(event Custom|AI_AbortAttack
  (if (Variables|/Game/MCS/Blueprints/MCSCharacter.MCSCharacter_C|GetIsAttacking? (Variables|References|GetCharacterRef))
    (Default|AttackReleased (Variables|References|GetCharacterRef))
    (Variables|Combat|SetTargetComboCount 0)
    (CallFunction|ResetAttack)))

(event EventBeginPlay)

(event EventTick
  (params (DeltaSeconds :type Float%20%28single-precision%29))
  ;[0.08618 0.631 1] Tick
)

(event EventOnPossess
  (params (PossessedPawn :type Pawn%20Object%20Reference))
  ;[1 1 1] Initialization
  (bind _asmcscharacter (Utilities|Casting|CastToMCSCharacter PossessedPawn))
  (Variables|References|SetCharacterRef _asmcscharacter))

(event EventIServerIsReady
  (bind _characterref (Variables|References|GetCharacterRef))
  ;[1 1 1] The server and clients are ready
  (Default|MULTIPlaySoundatLocation _characterref "/Game/MCS/Sounds/Bot/Spawn_Cue.Spawn_Cue" (Transformation|GetActorLocation _characterref))
  (Variables|/Game/MCS/Blueprints/MCSCharacter.MCSCharacter_C|SetInCombatMode (Variables|References|GetCharacterRef) true)
  (bind _returnvalue (AI|RunBehaviorTree "/Game/MCS/Blueprints/AI/MCSAI_BTree.MCSAI_BTree"))
  (if _returnvalue
    (Variables|/Script/Engine.Pawn|SetbUseControllerRotationYaw (Variables|References|GetCharacterRef) false)
    (Variables|/Script/Engine.CharacterMovementComponent|SetbUseControllerDesiredRotation (Variables|/Script/Engine.Character|GetCharacterMovement (Variables|References|GetCharacterRef)) true)
    (Variables|/Game/MCS/Blueprints/MCSCharacter.MCSCharacter_C|SetAttackDirection (Variables|References|GetCharacterRef) "NewEnumerator0")
    (else
      (Development|PrintString "AI: Could not run the behavior tree"))))

(fn ConstructionScript)

(fn SetRandomAttackDirection
  (switch int (Math|Random|RandomIntegerinRange 0 8)
    (:0
      (LocalVariables|SetRandomAttackDirection "NewEnumerator0"))
    (:1
      (LocalVariables|SetRandomAttackDirection "NewEnumerator6" :!label _label))
    (:2
      (goto _label))
    (:3
      (goto _label))
    (:4
      (LocalVariables|SetRandomAttackDirection "NewEnumerator5" :!label _label_2))
    (:5
      (goto _label_2))
    (:6
      (goto _label_2))
    (:7
      (LocalVariables|SetRandomAttackDirection "NewEnumerator2"))
    (:8
      (LocalVariables|SetRandomAttackDirection "NewEnumerator1")))
  (Variables|/Game/MCS/Blueprints/MCSCharacter.MCSCharacter_C|SetAttackDirection (Variables|References|GetCharacterRef) (LocalVariables|GetRandomAttackDirection))
  (Utilities|Struct|SetmembersinMCSAttackInfo (Variables|/Game/MCS/Blueprints/MCSCharacter.MCSCharacter_C|GetCurrentAttackInfo (Variables|References|GetCharacterRef)) (LocalVariables|GetRandomAttackDirection) (LocalVariables|GetRandomAttackDirection) 0.8))

(fn SetMovement
  (params (Direction :type MCSAttackDirection%20Enum :default "NewEnumerator8"))
  (LocalVariables|SetSpeed (Variables|/Game/MCS/Blueprints/MCSCharacter.MCSCharacter_C|GetDefaultCombatSpeed (Variables|References|GetCharacterRef)))
  (switch Utilities|FlowControl|Switch|SwitchonMCSAttackDirection Direction
    (:NewEnumerator8
      (bind _output_get (LocalVariables|SetSpeed 0.0))
      (bind _output_get_2 (LocalVariables|SetForwardAxisValue _output_get))
      (LocalVariables|SetRightAxisValue _output_get_2))
    (:NewEnumerator0
      (LocalVariables|SetForwardAxisValue 1.0)
      (LocalVariables|SetRightAxisValue 0.0))
    (:NewEnumerator1
      (LocalVariables|SetForwardAxisValue 1.0)
      (LocalVariables|SetRightAxisValue -1.0))
    (:NewEnumerator2
      (LocalVariables|SetForwardAxisValue 1.0)
      (LocalVariables|SetRightAxisValue 1.0))
    (:NewEnumerator7
      (LocalVariables|SetForwardAxisValue 1.0)
      (LocalVariables|SetRightAxisValue 0.0))
    (:NewEnumerator3
      (LocalVariables|SetForwardAxisValue 1.0)
      (LocalVariables|SetRightAxisValue -1.0))
    (:NewEnumerator4
      (LocalVariables|SetForwardAxisValue 1.0)
      (LocalVariables|SetRightAxisValue 1.0))
    (:NewEnumerator5
      (LocalVariables|SetForwardAxisValue 1.0)
      (LocalVariables|SetRightAxisValue -1.0))
    (:NewEnumerator6
      (LocalVariables|SetForwardAxisValue 1.0)
      (LocalVariables|SetRightAxisValue 1.0)))
  (Default|MoveForward (Variables|References|GetCharacterRef) (LocalVariables|GetForwardAxisValue))
  (Default|CLIENTSmoothSpeed (Variables|References|GetCharacterRef) (LocalVariables|GetSpeed) 15.0))