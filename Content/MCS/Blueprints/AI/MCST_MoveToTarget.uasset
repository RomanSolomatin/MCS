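; MCS behavior tree task that moves the AI character toward its target location.
; Each tick runs the parent logic, calls WalkReleased on the character if it is defending, then issues AIMoveTo using the combat radius as acceptance radius.
; The task finishes successfully when the move succeeds or when the pause-movement blackboard key is set; a failed move does not finish it.
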(event EventReceiveTickAI
  (params (OwnerController :type AI%20Controller%20Object%20Reference) (ControlledPawn :type Pawn%20Object%20Reference) (DeltaSeconds :type Float%20%28single-precision%29))
  (|CallParentFunction OwnerController ControlledPawn DeltaSeconds)
  (if (.IsDefending (Utilities|Struct|BreakMCSDefendInfo (Variables|/Game/MCS/Characters/MCSCharacter.MCSCharacter_C|GetDefendInfo (Variables|Default|GetAICharacterRef))))
    (Default|WalkReleased (Variables|Default|GetAICharacterRef)))
  (if (not (Class|BTFunctionLibrary|GetBlackboardValueasBool (Variables|Default|GetPauseMovementKey)))
    (AI|AIMoveTo (Variables|Default|GetAICharacterRef) (Variables|Default|GetTargetLocation) 0 (Variables|Default|GetCombatRadius) false
      (:OnSuccess
        (AI|BehaviorTree|FinishExecute true)))
    (else
      (AI|BehaviorTree|FinishExecute true))))