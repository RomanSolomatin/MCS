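; Behavior tree task that makes the AI character evade with a random jump while attacking, or a random roll otherwise.
; It pauses blackboard movement, clears focus, sets directional velocity and attack direction, then simulates jump or crouch input.
; After a delay it releases the input, resumes movement, refocuses the target and finishes as failed, as it does when already falling or rolling.
; The GetLaunchVector launch path is never run.
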(event Custom|RollRight
  (bind _aicharacterref (Variables|Default|GetAICharacterRef))
  ;[1 1 1] Random Roll
  (Variables|/Script/Engine.MovementComponent|SetVelocity (Pawn|GetMovementComponent _aicharacterref) (* (Transformation|GetActorRightVector _aicharacterref) 1e+03))
  (Variables|/Game/MCS/Characters/MCSCharacter.MCSCharacter_C|SetAttackDirection (Variables|Default|GetAICharacterRef) "NewEnumerator6")
  (Default|CrouchPressed (Variables|Default|GetAICharacterRef))
  (Utilities|FlowControl|Delay (Variables|Default|GetDelayAmount))
  (Default|CrouchReleased (Variables|Default|GetAICharacterRef))
  (Class|BTFunctionLibrary|SetBlackboardValueasBool (Variables|Default|GetPauseMovementKey) false)
  (AI|SetFocus (Variables|Default|GetAIControllerRef) (Variables|Default|GetTargetRef))
  (AI|BehaviorTree|FinishExecute false))

(event Custom|JumpLeft
  (bind _aicharacterref (Variables|Default|GetAICharacterRef))
  (Variables|/Script/Engine.MovementComponent|SetVelocity (Pawn|GetMovementComponent _aicharacterref) (* (Transformation|GetActorRightVector _aicharacterref) -6.8e+02))
  (Variables|/Game/MCS/Characters/MCSCharacter.MCSCharacter_C|SetAttackDirection (Variables|Default|GetAICharacterRef) "NewEnumerator5")
  (Default|JumpPressed (Variables|Default|GetAICharacterRef))
  (Utilities|FlowControl|Delay (Math|Random|RandomFloatinRange 0.1 0.3))
  (Default|JumpReleased (Variables|Default|GetAICharacterRef))
  (Class|BTFunctionLibrary|SetBlackboardValueasBool (Variables|Default|GetPauseMovementKey) false)
  (AI|SetFocus (Variables|Default|GetAIControllerRef) (Variables|Default|GetTargetRef))
  (AI|BehaviorTree|FinishExecute false))

(event Custom|RandomRoll
  ;[1 1 1] Random Roll
  (Class|BTFunctionLibrary|SetBlackboardValueasBool (Variables|Default|GetPauseMovementKey) true)
  (AI|ClearFocus (Variables|Default|GetAIControllerRef))
  (switch int (Math|Random|RandomIntegerinRange 0 2)
    (:0
      (CallFunction|RollLeft))
    (:1
      (CallFunction|RollRight))
    (:2
      (CallFunction|RollBack))))

(event Custom|JumpForward
  (bind _aicharacterref (Variables|Default|GetAICharacterRef))
  (Variables|/Script/Engine.MovementComponent|SetVelocity (Pawn|GetMovementComponent _aicharacterref) (* (Transformation|GetActorForwardVector _aicharacterref) 6e+02))
  (Variables|/Game/MCS/Characters/MCSCharacter.MCSCharacter_C|SetAttackDirection (Variables|Default|GetAICharacterRef) "NewEnumerator0")
  (Default|JumpPressed (Variables|Default|GetAICharacterRef))
  (Utilities|FlowControl|Delay (Math|Random|RandomFloatinRange 0.1 0.3))
  (Default|JumpReleased (Variables|Default|GetAICharacterRef))
  (Class|BTFunctionLibrary|SetBlackboardValueasBool (Variables|Default|GetPauseMovementKey) false)
  (AI|SetFocus (Variables|Default|GetAIControllerRef) (Variables|Default|GetTargetRef))
  (AI|BehaviorTree|FinishExecute false))

(event Custom|RollLeft
  (bind _aicharacterref (Variables|Default|GetAICharacterRef))
  ;[1 1 1] Random Roll
  (Variables|/Script/Engine.MovementComponent|SetVelocity (Pawn|GetMovementComponent _aicharacterref) (* (Transformation|GetActorRightVector _aicharacterref) -1e+03))
  (Variables|/Game/MCS/Characters/MCSCharacter.MCSCharacter_C|SetAttackDirection (Variables|Default|GetAICharacterRef) "NewEnumerator5")
  (Default|CrouchPressed (Variables|Default|GetAICharacterRef))
  (Utilities|FlowControl|Delay (Variables|Default|GetDelayAmount))
  (Default|CrouchReleased (Variables|Default|GetAICharacterRef))
  (Class|BTFunctionLibrary|SetBlackboardValueasBool (Variables|Default|GetPauseMovementKey) false)
  (AI|SetFocus (Variables|Default|GetAIControllerRef) (Variables|Default|GetTargetRef))
  (AI|BehaviorTree|FinishExecute false))

(event Custom|RollBack
  (bind _aicharacterref (Variables|Default|GetAICharacterRef))
  ;[1 1 1] Random Roll
  (Variables|/Script/Engine.MovementComponent|SetVelocity (Pawn|GetMovementComponent _aicharacterref) (* (Transformation|GetActorForwardVector _aicharacterref) -1e+03))
  (Variables|/Game/MCS/Characters/MCSCharacter.MCSCharacter_C|SetAttackDirection (Variables|Default|GetAICharacterRef) "NewEnumerator7")
  (Default|CrouchPressed (Variables|Default|GetAICharacterRef))
  (Utilities|FlowControl|Delay (Variables|Default|GetDelayAmount))
  (Default|CrouchReleased (Variables|Default|GetAICharacterRef))
  (Class|BTFunctionLibrary|SetBlackboardValueasBool (Variables|Default|GetPauseMovementKey) false)
  (AI|SetFocus (Variables|Default|GetAIControllerRef) (Variables|Default|GetTargetRef))
  (AI|BehaviorTree|FinishExecute false))

(event Custom|RandomJump
  (Class|BTFunctionLibrary|SetBlackboardValueasBool (Variables|Default|GetPauseMovementKey) true)
  (AI|ClearFocus (Variables|Default|GetAIControllerRef))
  (switch int (Math|Random|RandomIntegerinRange 0 2)
    (:0
      (CallFunction|JumpRight))
    (:1
      (CallFunction|JumpLeft))
    (:2
      (CallFunction|JumpForward))))

(event Custom|JumpRight
  (bind _aicharacterref (Variables|Default|GetAICharacterRef))
  (Variables|/Script/Engine.MovementComponent|SetVelocity (Pawn|GetMovementComponent _aicharacterref) (* (Transformation|GetActorRightVector _aicharacterref) 6e+02))
  (Variables|/Game/MCS/Characters/MCSCharacter.MCSCharacter_C|SetAttackDirection (Variables|Default|GetAICharacterRef) "NewEnumerator6")
  (Default|JumpPressed (Variables|Default|GetAICharacterRef))
  (Utilities|FlowControl|Delay (Math|Random|RandomFloatinRange 0.1 0.3))
  (Default|JumpReleased (Variables|Default|GetAICharacterRef))
  (Class|BTFunctionLibrary|SetBlackboardValueasBool (Variables|Default|GetPauseMovementKey) false)
  (AI|SetFocus (Variables|Default|GetAIControllerRef) (Variables|Default|GetTargetRef))
  (AI|BehaviorTree|FinishExecute false))

(event EventReceiveExecuteAI
  (params (OwnerController :type AI%20Controller%20Object%20Reference) (ControlledPawn :type Pawn%20Object%20Reference))
  (|CallParentFunction OwnerController ControlledPawn)
  (if (Utilities|Struct|BreakMCSAttackInfo (Variables|/Game/MCS/Characters/MCSCharacter.MCSCharacter_C|GetCurrentAttackInfo (Variables|Default|GetAICharacterRef)))
    (if (not (AI|Components|NavMovement|IsFalling (Variables|/Script/Engine.Character|GetCharacterMovement (Variables|Default|GetAICharacterRef))))
      (CallFunction|RandomJump)
      (else
        (AI|BehaviorTree|FinishExecute false :!label _label)))
    (elif (not (.IsRolling (Utilities|Struct|BreakMCSPlayerMovement (Variables|/Game/MCS/Characters/MCSCharacter.MCSCharacter_C|GetPlayerMovement (Variables|Default|GetAICharacterRef)))))
      (CallFunction|RandomRoll)
      (else
        (goto _label)))))

(fn GetLaunchVector
  (switch int (Math|Random|RandomIntegerinRange 0 2)
    (:0
      (LocalVariables|SetImpulseVector (Transformation|GetActorForwardVector (Variables|Default|GetAICharacterRef))))
    (:1
      (LocalVariables|SetImpulseVector (Transformation|GetActorRightVector (Variables|Default|GetAICharacterRef))))
    (:2
      (LocalVariables|SetImpulseVector (* (Transformation|GetActorRightVector (Variables|Default|GetAICharacterRef)) -1.0))))
  (LocalVariables|SetVector (Math|Vector|MakeVector (.X (Math|Vector|BreakVector (Math|Vector|RotateVectorAroundAxis (* (LocalVariables|GetImpulseVector) 6e+02) (Math|Random|RandomFloatinRange -3e+01 3e+01) "0, 0,1.000000"))) (.Y (Math|Vector|BreakVector (Math|Vector|RotateVectorAroundAxis (* (LocalVariables|GetImpulseVector) 6e+02) (Math|Random|RandomFloatinRange -3e+01 3e+01) "0, 0,1.000000"))) (Math|Random|RandomFloatinRange 6e+02 1.6e+03)))
  (return (LocalVariables|GetVector)))