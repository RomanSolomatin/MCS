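; MCST_Attack is a behavior tree task that makes an AI character perform a random attack on its target.
; After the parent task runs, it requires a valid AI controller, a target within combat radius, and the character no more than 100 units above the ground.
; Passing triggers the controller's random attack and finishes successfully; failing the range or height check aborts the attack and fails the task.
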(event EventReceiveExecuteAI
  (params (OwnerController :type AI%20Controller%20Object%20Reference) (ControlledPawn :type Pawn%20Object%20Reference))
  (|CallParentFunction OwnerController ControlledPawn)
  (Utilities|IsValid (Variables|Default|GetAIControllerRef)
    (:Is%20Valid
      (if (and (<= (Variables|Default|GetDistanceToTarget) (Variables|Default|GetCombatRadius)) (<= (Variables|/Game/MCS/Blueprints/MCSCharacter.MCSCharacter_C|GetCurrentDistanceToGround (Variables|Default|GetAICharacterRef)) 1e+02))
        (Default|AIRandomAttack (Variables|Default|GetAIControllerRef))
        (AI|BehaviorTree|FinishExecute true)
        (else
          (Default|AIAbortAttack (Variables|Default|GetAIControllerRef))
          (AI|BehaviorTree|FinishExecute false))))))