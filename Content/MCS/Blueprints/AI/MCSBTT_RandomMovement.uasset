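; Behavior tree task that moves an AI around its closest enemy during combat, backing away inside attack radius and otherwise mostly advancing with occasional strafes.
; A delta-time timer re-rolls the movement choice at short random intervals.
; Each execution updates the in-combat-range and can-attack blackboard keys, allowing slight slack on attack radius, then finishes immediately, so movement advances per run rather than through a latent action.
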(event EventReceiveExecuteAI
  (params (OwnerController :type AI%20Controller%20Object%20Reference) (ControlledPawn :type Pawn%20Object%20Reference))
  (|CallParentFunction OwnerController ControlledPawn)
  ;[1 1 1] Update combat range key.  Leave branch if out of range.
  (bind _output_get (Variables|Default|SetInCombatRange (<= (Variables|Default|GetClosestEnemyDistance) (Variables|Default|GetCombatRadius))))
  (Class|BTFunctionLibrary|SetBlackboardValueasBool (Variables|Blackboard|GetInCombatRangeKey) _output_get)
  (if (<= (Variables|Default|GetClosestEnemyDistance) (Class|BTFunctionLibrary|GetBlackboardValueasFloat (Variables|Blackboard|GetAttackRadiusKey)))
    (CallFunction|MoveBack false)
    (Blackboard|UpdateCanAttack)
    (else
      (Variables|Default|SetCurrentTimer (+ (Utilities|Time|GetWorldDeltaSeconds) (Variables|Default|GetCurrentTimer)))
      (if (>= (Variables|Default|GetCurrentTimer) (Variables|Default|GetRandomTime))
        (Variables|Default|SetCurrentTimer 0.0)
        (Variables|Default|SetRandomTime (Math|Random|RandomFloatinRange 0.5 1.5))
        (Variables|Default|SetRandomMovementID (Math|Random|RandomIntegerinRange 0 9))
        (Blackboard|UpdateCanAttack)
        (else
          (switch int (Variables|Default|GetRandomMovementID)
            (:Default
              (CallFunction|MoveForward false))
            (:0
              (CallFunction|StrafeRight false))
            (:1
              (CallFunction|StrafeLeft false)))
          (Blackboard|UpdateCanAttack))))))

(fn UpdateCanAttack
  (bind _output_get (LocalVariables|SetCanAttack (< (Variables|Default|GetClosestEnemyDistance) (+ (Class|BTFunctionLibrary|GetBlackboardValueasFloat (Variables|Blackboard|GetAttackRadiusKey)) 5e+01))))
  (Class|BTFunctionLibrary|SetBlackboardValueasBool (Variables|Blackboard|GetCanAttackKey) _output_get)
  (AI|BehaviorTree|FinishExecute true))