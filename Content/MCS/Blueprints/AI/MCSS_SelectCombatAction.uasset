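; Behavior tree service that picks an AI character's combat state based on whether its target is attacking.
; Each tick it caches the controller, pawn and the target character read from the Blackboard.
; While the target attacks, a weighted random roll chooses among three states, favoring the default one that is also used otherwise.
; SetAIState stores the choice and writes it to the Blackboard state key.
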(event EventReceiveTickAI
  (params (OwnerController :type AI%20Controller%20Object%20Reference) (ControlledPawn :type Pawn%20Object%20Reference) (DeltaSeconds :type Float%20%28single-precision%29))
  (Variables|Globals|SetDeltaTime DeltaSeconds)
  (bind _asmcsaicontroller (Utilities|Casting|CastToMCSAIController OwnerController))
  (Variables|AI|SetAIControllerRef _asmcsaicontroller)
  (bind _asmcscharacter (Utilities|Casting|CastToMCSCharacter ControlledPawn))
  (Variables|AI|SetAICharacterRef _asmcscharacter)
  (bind _asmcscharacter_2 (Utilities|Casting|CastToMCSCharacter (Class|BTFunctionLibrary|GetBlackboardValueasObject (Variables|Keys|GetTargetToFollowKey))))
  (Variables|Target|SetTargetRef _asmcscharacter_2)
  (if (Variables|/Game/MCS/Blueprints/MCSCharacter.MCSCharacter_C|GetIsAttacking? (Variables|Target|GetTargetRef))
    (switch int (Math|Random|RandomIntegerinRange 0 8)
      (:Default
        (CallFunction|SetAIState "NewEnumerator2"))
      (:0
        (CallFunction|SetAIState "NewEnumerator4"))
      (:1
        (CallFunction|SetAIState "NewEnumerator3" :!label _label))
      (:2
        (goto _label))
      (:3
        (goto _label)))
    (else
      (CallFunction|SetAIState "NewEnumerator2"))))

(fn SetAIState
  (params (State :type MCSAIState%20Enum :default "NewEnumerator0"))
  (bind _output_get (Variables|AI|SetAIState State))
  (Class|BTFunctionLibrary|SetBlackboardValueasEnum (Variables|Keys|GetAIStateKey) _output_get))