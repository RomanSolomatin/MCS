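; Behavior tree task that makes an AI MCSCharacter chase the blackboard's TargetToFollow character until it is within attack range.
; Each tick it reads the target, smoothly rotates toward it while keeping current pitch, and ramps to combat speed if max walk speed is zero.
; It also reissues AIMoveTo every tick using the character's CombatRadius, setting InAttackRange and finishing on success, with no failure branch.
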(event EventReceiveTickAI
  (params (OwnerController :type AI%20Controller%20Object%20Reference) (ControlledPawn :type Pawn%20Object%20Reference) (DeltaSeconds :type Float%20%28single-precision%29))
  (Variables|Default|SetDeltaTime DeltaSeconds)
  (if (== (Variables|References|GetAIControllerRef) 0)
    (bind _asmcsaicontroller (Utilities|Casting|CastToMCSAIController OwnerController))
    (bind _output_get (Variables|References|SetAIControllerRef _asmcsaicontroller))
    (bind _asmcscharacter (Utilities|Casting|CastToMCSCharacter (Pawn|GetControlledPawn _output_get)))
    (Variables|References|SetAICharacterRef _asmcscharacter))
  (bind _asmcscharacter_2 (Utilities|Casting|CastToMCSCharacter (Class|BTFunctionLibrary|GetBlackboardValueasObject (Variables|Keys|GetTargetToFollow))))
  (Variables|References|SetTargetRef _asmcscharacter_2)
  (CallFunction|TrackTarget)
  (if (<= (Variables|/Script/Engine.CharacterMovementComponent|GetMaxWalkSpeed (Variables|/Script/Engine.Character|GetCharacterMovement (Variables|References|GetAICharacterRef))) 0.0)
    (Default|CLIENTSmoothSpeed (Variables|References|GetAICharacterRef) (Variables|/Game/MCS/Blueprints/MCSCharacter.MCSCharacter_C|GetDefaultCombatSpeed (Variables|References|GetAICharacterRef)) 15.0))
  (AI|AIMoveTo (Variables|References|GetAICharacterRef) "0, 0, 0" (Variables|References|GetTargetRef) (Variables|/Game/MCS/Blueprints/MCSCharacter.MCSCharacter_C|GetCombatRadius (Variables|References|GetAICharacterRef)) false
    (:then
      (Variables|Default|SetTargetDistance (Transformation|GetDistanceTo (Variables|References|GetAICharacterRef) (Variables|References|GetTargetRef))))
    (:OnSuccess
      (Class|BTFunctionLibrary|SetBlackboardValueasBool (Variables|Keys|GetInAttackRange) true)
      (AI|BehaviorTree|FinishExecute true))))

(fn TrackTarget
  (bind _aicharacterref (Variables|References|GetAICharacterRef))
  (bind _aicharacterref_2 (Variables|References|GetAICharacterRef))
  (bind _targetref (Variables|References|GetTargetRef))
  (bind _returnvalue (Transformation|GetActorLocation _targetref))
  (bind _returnvalue_2 (Transformation|GetActorRotation _aicharacterref_2))
  (bind _returnvalue_3 (Transformation|GetActorLocation _aicharacterref))
  (bind _returnvalue_4 (Math|Rotator|FindLookatRotation _returnvalue_3 _returnvalue))
  (bind (_roll _pitch _yaw) (Math|Rotator|BreakRotator _returnvalue_4))
  (Transformation|SetActorRotation (Variables|References|GetAICharacterRef) (Math|Interpolation|RInterpTo _returnvalue_2 (Math|Rotator|MakeRotator _roll (.Pitch (Math|Rotator|BreakRotator _returnvalue_2)) _yaw) (Variables|Default|GetDeltaTime) 15.0)))