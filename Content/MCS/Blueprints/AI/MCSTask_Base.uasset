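; Base behavior tree task for MCS AI characters that caches combat data about the followed target and updates the AI state.
; On execute and tick it caches the controller and character, then runs UpdateValues.
; UpdateValues reads the blackboard target and stores its location, distance, attack and movement info.
; It writes one of three states to the blackboard: target within combat radius plus a margin, farther away, or invalid or dead.
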(event EventReceiveTickAI
  (params (OwnerController :type AI%20Controller%20Object%20Reference) (ControlledPawn :type Pawn%20Object%20Reference) (DeltaSeconds :type Float%20%28single-precision%29))
  (Variables|Globals|SetDeltaTime DeltaSeconds)
  (if (== (Variables|References|GetAIControllerRef) 0)
    (bind _asmcsaicontroller (Utilities|Casting|CastToMCSAIController OwnerController))
    (Variables|References|SetAIControllerRef _asmcsaicontroller)
    (bind _asmcscharacter (Utilities|Casting|CastToMCSCharacter ControlledPawn))
    (Variables|References|SetAICharacterRef _asmcscharacter))
  (CallFunction|UpdateValues))

(event EventReceiveExecuteAI
  (params (OwnerController :type AI%20Controller%20Object%20Reference) (ControlledPawn :type Pawn%20Object%20Reference))
  (if (== (Variables|References|GetAIControllerRef) 0)
    (bind _asmcsaicontroller (Utilities|Casting|CastToMCSAIController OwnerController))
    (Variables|References|SetAIControllerRef _asmcsaicontroller)
    (bind _asmcscharacter (Utilities|Casting|CastToMCSCharacter ControlledPawn))
    (Variables|References|SetAICharacterRef _asmcscharacter))
  (CallFunction|UpdateValues))

(fn UpdateValues
  (bind _targettofollowkey (Variables|Keys|GetTargetToFollowKey))
  (bind _returnvalue (Class|BTFunctionLibrary|GetBlackboardValueasObject _targettofollowkey))
  (Variables|AI|SetAIState (Utilities|Enum|ByteToEnumMCSAIState (Class|BTFunctionLibrary|GetBlackboardValueasEnum (Variables|Keys|GetAIStateKey))))
  (Utilities|IsValid _returnvalue
    (:Is%20Valid
      (bind _asmcscharacter (Utilities|Casting|CastToMCSCharacter _returnvalue)
        (:then
          (bind _output_get (Variables|References|SetTargetRef _asmcscharacter))
          (Utilities|IsValid _output_get
            (:Is%20Valid
              (if (not (Variables|/Game/MCS/Blueprints/MCSCharacter.MCSCharacter_C|GetIsDead? (Variables|References|GetTargetRef)))
                (Variables|AI|SetCombatRadius (Variables|/Game/MCS/Blueprints/MCSCharacter.MCSCharacter_C|GetDefaultCombatRadius (Variables|References|GetAICharacterRef)))
                (bind _output_get_2 (Variables|AI|SetAILocation (Transformation|GetActorLocation (Variables|References|GetAICharacterRef))))
                (Variables|AI|SetAIXYLocation (Math|Vector|MakeVector (.X (Math|Vector|BreakVector _output_get_2)) (.Y (Math|Vector|BreakVector _output_get_2)) 0.0))
                (bind _output_get_3 (Variables|Target|SetTargetLocation (Transformation|GetActorLocation (Variables|References|GetTargetRef))))
                (Variables|Target|SetTargetXYLocation (Math|Vector|MakeVector (.X (Math|Vector|BreakVector _output_get_3)) (.Y (Math|Vector|BreakVector _output_get_3)) 0.0))
                (bind _output_get_4 (Variables|AI|SetLookAtRotation (Math|Rotator|FindLookatRotation (Variables|AI|GetAILocation) (Variables|Target|GetTargetLocation))))
                (Variables|AI|SetLookAtVector (Math|Vector|GetForwardVector _output_get_4))
                (Variables|Target|SetDistanceToTarget (Math|Vector|VectorLength (- (Variables|AI|GetAILocation) (Variables|Target|GetTargetLocation))))
                (Variables|AI|SetCurrentSpeed (Variables|/Script/Engine.CharacterMovementComponent|GetMaxWalkSpeed (Variables|/Script/Engine.Character|GetCharacterMovement (Variables|References|GetAICharacterRef))))
                (Variables|Target|SetTargetIsAttacking (Variables|/Game/MCS/Blueprints/MCSCharacter.MCSCharacter_C|GetIsAttacking? (Variables|References|GetTargetRef)))
                (bind _output_get_5 (Variables|Target|SetTargetAttackInfo (Variables|/Game/MCS/Blueprints/MCSCharacter.MCSCharacter_C|GetCurrentAttackInfo (Variables|References|GetTargetRef))))
                (Variables|Target|SetTargetAttackDirection (.CurrentSwingDirection (Utilities|Struct|BreakMCSAttackInfo _output_get_5)))
                (Variables|Target|SetTargetMovementInfo (Variables|/Game/MCS/Blueprints/MCSCharacter.MCSCharacter_C|GetPlayerMovement (Variables|References|GetTargetRef)))
                (Variables|Target|SetTargetMovementDirection (Variables|/Game/MCS/Blueprints/MCSCharacter.MCSCharacter_C|GetAttackDirection (Variables|References|GetTargetRef)))
                (if (<= (Variables|Target|GetDistanceToTarget) (+ (Variables|AI|GetCombatRadius) 5e+01))
                  (CallFunction|SetAIState "NewEnumerator5")
                  (else
                    (CallFunction|SetAIState "NewEnumerator1")))
                (else
                  (CallFunction|SetAIState "NewEnumerator0" :!label _label))))
            (:Is%20Not%20Valid
              (goto _label))))
        (:CastFailed
          (goto _label))))
    (:Is%20Not%20Valid
      (goto _label))))

(fn SetAIState
  (params (State :type MCSAIState%20Enum :default "NewEnumerator0"))
  (bind _output_get (Variables|AI|SetAIState State))
  (Class|BTFunctionLibrary|SetBlackboardValueasEnum (Variables|Keys|GetAIStateKey) _output_get))