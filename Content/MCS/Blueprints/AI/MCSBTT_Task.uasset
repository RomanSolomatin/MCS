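; Behavior Tree task for MCS combat bots that provides shared attack, roll, jump, walk and strafe actions.
; Execute, tick and abort events cache controller, pawn and the blackboard's closest enemy, then update enemy distance and derive AttackDirection from local-space velocity.
; Moves focus the enemy and AI-move a short step; most actions finish the task themselves.
; Rolls randomize direction when stationary, then flip strafes or sidestep an attacking enemy.
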(event EventReceiveExecuteAI
  (params (OwnerController :type AI%20Controller%20Object%20Reference) (ControlledPawn :type Pawn%20Object%20Reference))
  ;[1 1 1] Update references / Distance to enemy (if one exists) / the current enemy location / and set the "MCSAttackDirection" enumerator to the current movement of the bot
  (bind (_castaicontroller _castaipawn) (References|CasttoAI OwnerController ControlledPawn))
  (Variables|References|SetAIController _castaicontroller)
  (Variables|References|SetAIPawn _castaipawn)
  (bind _enemy (References|CasttoEnemy))
  (Variables|References|SetCurrentEnemy _enemy)
  (Blackboard|UpdateDistancetoEnemy)
  (Movement|SetCurrentDirection))

(event EventReceiveExecute
  (params (OwnerActor :type Actor%20Object%20Reference))
  ;[1 1 1] Update references / Distance to enemy (if one exists) / the current enemy location / and set the "MCSAttackDirection" enumerator to the current movement of the bot
  (bind _asmcsbot (Utilities|Casting|CastToMCSBot OwnerActor)
    (:then
      (Variables|References|SetAIPawn _asmcsbot)
      (bind _enemy (References|CasttoEnemy))
      (Variables|References|SetCurrentEnemy _enemy)
      (Blackboard|UpdateDistancetoEnemy)
      (Movement|SetCurrentDirection))
    (:CastFailed
      (Development|PrintString "MCSBTT_Task <Event Receive Execute>: Cast to MCSBot FAILED"))))

(event EventTick
  (params (OwnerActor :type Actor%20Object%20Reference) (DeltaSeconds :type Float%20%28single-precision%29))
  ;[1 1 1] Update references / Distance to enemy (if one exists) / the current enemy location / and set the "MCSAttackDirection" enumerator to the current movement of the bot
  (bind _asmcsbot (Utilities|Casting|CastToMCSBot OwnerActor)
    (:then
      (Variables|References|SetAIPawn _asmcsbot)
      (bind _enemy (References|CasttoEnemy))
      (Variables|References|SetCurrentEnemy _enemy)
      (Blackboard|UpdateDistancetoEnemy)
      (Movement|SetCurrentDirection))
    (:CastFailed
      (Development|PrintString "MCSBTT_Task <Event Receive Tick>: Cast to MCSBot FAILED"))))

(event EventReceiveTickAI
  (params (OwnerController :type AI%20Controller%20Object%20Reference) (ControlledPawn :type Pawn%20Object%20Reference) (DeltaSeconds :type Float%20%28single-precision%29))
  ;[1 1 1] Update references / Distance to enemy (if one exists) / the current enemy location / and set the "MCSAttackDirection" enumerator to the current movement of the bot
  (bind (_castaicontroller _castaipawn) (References|CasttoAI OwnerController ControlledPawn))
  (Variables|References|SetAIController _castaicontroller)
  (Variables|References|SetAIPawn _castaipawn)
  (bind _enemy (References|CasttoEnemy))
  (Variables|References|SetCurrentEnemy _enemy)
  (Blackboard|UpdateDistancetoEnemy)
  (Movement|SetCurrentDirection))

(event EventReceiveAbortAI
  (params (OwnerController :type AI%20Controller%20Object%20Reference) (ControlledPawn :type Pawn%20Object%20Reference))
  ;[1 1 1] Update references / Distance to enemy (if one exists) / the current enemy location / and set the "MCSAttackDirection" enumerator to the current movement of the bot
  (bind (_castaicontroller _castaipawn) (References|CasttoAI OwnerController ControlledPawn))
  (Variables|References|SetAIController _castaicontroller)
  (Variables|References|SetAIPawn _castaipawn)
  (bind _enemy (References|CasttoEnemy))
  (Variables|References|SetCurrentEnemy _enemy)
  (Blackboard|UpdateDistancetoEnemy)
  (Movement|SetCurrentDirection))

(event EventReceiveAbort
  (params (OwnerActor :type Actor%20Object%20Reference))
  ;[1 1 1] Update references / Distance to enemy (if one exists) / the current enemy location / and set the "MCSAttackDirection" enumerator to the current movement of the bot
  (bind _asmcsbot (Utilities|Casting|CastToMCSBot OwnerActor)
    (:then
      (Variables|References|SetAIPawn _asmcsbot)
      (bind _enemy (References|CasttoEnemy))
      (Variables|References|SetCurrentEnemy _enemy)
      (Blackboard|UpdateDistancetoEnemy)
      (Movement|SetCurrentDirection))
    (:CastFailed
      (Development|PrintString "MCSBTT_Task <Event Receive Abort>: Cast to MCSBot FAILED"))))

(event Custom|StrafeRight
  (params (Walk :type Boolean))
  ;[1 1 1] Strafe walk/run
  (Variables|/Game/MCS/Blueprints/MCSCharacter.MCSCharacter_C|SetAttackDirection (Variables|References|GetAIPawn) "NewEnumerator5")
  (AI|SetFocus (Variables|References|GetAIController) (Variables|References|GetCurrentEnemy))
  (if Walk
    (Default|AIWalk (Variables|References|GetAIPawn)))
  (AI|AIMoveTo (Variables|References|GetAIPawn) (+ (* (Transformation|GetActorRightVector (Variables|References|GetAIPawn)) 5e+01) (Transformation|GetWorldLocation (Variables|/Script/Engine.Character|GetMesh (Variables|References|GetAIPawn)))) 0 5.0 false
    (:then
      (AI|BehaviorTree|FinishExecute true))))

(event Custom|StrafeLeft
  (params (Walk :type Boolean))
  ;[1 1 1] Strafe walk/run
  (Variables|/Game/MCS/Blueprints/MCSCharacter.MCSCharacter_C|SetAttackDirection (Variables|References|GetAIPawn) "NewEnumerator6")
  (AI|SetFocus (Variables|References|GetAIController) (Variables|References|GetCurrentEnemy))
  (if Walk
    (Default|AIWalk (Variables|References|GetAIPawn)))
  (AI|AIMoveTo (Variables|References|GetAIPawn) (+ (* (Transformation|GetActorRightVector (Variables|References|GetAIPawn)) -5e+01) (Transformation|GetWorldLocation (Variables|/Script/Engine.Character|GetMesh (Variables|References|GetAIPawn)))) 0 5.0 false
    (:then
      (AI|BehaviorTree|FinishExecute true))))

(event Custom|MoveForward
  (params (Walk :type Boolean))
  ;[1 1 1] Walk/Run  forward/back
  (Variables|/Game/MCS/Blueprints/MCSCharacter.MCSCharacter_C|SetAttackDirection (Variables|References|GetAIPawn) "NewEnumerator0")
  (AI|SetFocus (Variables|References|GetAIController) (Variables|References|GetCurrentEnemy))
  (if Walk
    (Default|AIWalk (Variables|References|GetAIPawn)))
  (AI|AIMoveTo (Variables|References|GetAIPawn) (+ (* (Transformation|GetActorForwardVector (Variables|References|GetAIPawn)) 5e+01) (Transformation|GetWorldLocation (Variables|/Script/Engine.Character|GetMesh (Variables|References|GetAIPawn)))) 0 5.0 false
    (:then
      (AI|BehaviorTree|FinishExecute true))))

(event Custom|MoveBack
  (params (Walk :type Boolean))
  ;[1 1 1] Walk/Run  forward/back
  (Variables|/Game/MCS/Blueprints/MCSCharacter.MCSCharacter_C|SetAttackDirection (Variables|References|GetAIPawn) "NewEnumerator7")
  (AI|SetFocus (Variables|References|GetAIController) (Variables|References|GetCurrentEnemy))
  (if Walk
    (Default|AIWalk (Variables|References|GetAIPawn)))
  (AI|AIMoveTo (Variables|References|GetAIPawn) (+ (* (Transformation|GetActorForwardVector (Variables|References|GetAIPawn)) -5e+01) (Transformation|GetWorldLocation (Variables|/Script/Engine.Character|GetMesh (Variables|References|GetAIPawn)))) 0 5.0 false
    (:then
      (AI|BehaviorTree|FinishExecute true))))

(event Custom|Roll
  ;[1 1 1] Rolling
  (if (> (Math|Vector|VectorLength (Transformation|GetVelocity (Variables|References|GetAIPawn))) 0.0) ; Is  the BOT moving?
    _
    (else
      (Movement|SelectRandomRollDirection)))
  (Movement|ReverseDirection)
  (Default|AIRollMulticast (Variables|References|GetAIPawn))
  (AI|BehaviorTree|FinishExecute true))

(event Custom|Attack
  ;[1 1 1] Attacking
  (Default|AIAttack (Variables|References|GetAIPawn))
  (Utilities|FlowControl|Delay 1.0)
  (AI|BehaviorTree|FinishExecute true))

(event Custom|AbortAttack
  ;[1 1 1] Attacking
)

(event Custom|Jump
  (params (Duration :type Float%20%28single-precision%29))
  ;[1 1 1] Jumping
  (Default|AIJump (Variables|References|GetAIPawn) 0.0))

(event Custom|AttackInPlace
  ;[1 1 1] Attacking
  ;;[1 0 0] TESTING
  (Default|AIAttackinDirectionMulticast (Variables|References|GetAIPawn) "NewEnumerator5")
  (AI|BehaviorTree|FinishExecute true))

(fn UpdateDistancetoEnemy
  (Utilities|IsValid (Variables|References|GetCurrentEnemy)
    (:Is%20Valid
      (Variables|Movement|SetClosestEnemyDistance (Transformation|GetDistanceTo (Variables|References|GetAIPawn) (Variables|References|GetCurrentEnemy)))
      (return))))

(fn SetCurrentDirection
  (if (Utilities|IsValid (Variables|References|GetAIPawn))
    (bind _output_get (LocalVariables|SetVelocityVector (Math|Transform|InverseTransformDirection (Transformation|GetActorTransform (Variables|References|GetAIPawn)) (Math|Vector|Normalize (Transformation|GetVelocity (Variables|References|GetAIPawn))))))
    (if (> (Math|Vector|VectorLength _output_get) 0.0) ; Is the AI moving?
      (if (> (.x (LocalVariables|GetVelocityVector)) 0.9)
        (Variables|/Game/MCS/Blueprints/MCSCharacter.MCSCharacter_C|SetAttackDirection (Variables|References|GetAIPawn) "NewEnumerator0")
        (return)
        (elif (< (.x (LocalVariables|GetVelocityVector)) -0.9)
          (Variables|/Game/MCS/Blueprints/MCSCharacter.MCSCharacter_C|SetAttackDirection (Variables|References|GetAIPawn) "NewEnumerator7")
          (return)
          (elif (> (.y (LocalVariables|GetVelocityVector)) 0.9)
            (Variables|/Game/MCS/Blueprints/MCSCharacter.MCSCharacter_C|SetAttackDirection (Variables|References|GetAIPawn) "NewEnumerator5")
            (return)
            (elif (< (.y (LocalVariables|GetVelocityVector)) -0.9)
              (Variables|/Game/MCS/Blueprints/MCSCharacter.MCSCharacter_C|SetAttackDirection (Variables|References|GetAIPawn) "NewEnumerator6")
              (return)))))
      (else
        (Variables|/Game/MCS/Blueprints/MCSCharacter.MCSCharacter_C|SetAttackDirection (Variables|References|GetAIPawn) "NewEnumerator8")
        (return)))
    (else
      (return))))

(fn ReverseDirection
  (if (and (Utilities|Enum|Equal(Enum) (Variables|/Game/MCS/Blueprints/MCSCharacter.MCSCharacter_C|GetAttackDirection (Variables|References|GetAIPawn)) "NewEnumerator0") (Variables|/Game/MCS/Blueprints/MCSCharacter.MCSCharacter_C|GetIsAttacking? (Variables|References|GetCurrentEnemy)))
    (switch int (Math|Random|RandomIntegerinRange 0 1)
      (:0
        (Variables|/Game/MCS/Blueprints/MCSCharacter.MCSCharacter_C|SetAttackDirection (Variables|References|GetAIPawn) "NewEnumerator5"))
      (:1
        (Variables|/Game/MCS/Blueprints/MCSCharacter.MCSCharacter_C|SetAttackDirection (Variables|References|GetAIPawn) "NewEnumerator6")))
    (elif (Utilities|Enum|Equal(Enum) (Variables|/Game/MCS/Blueprints/MCSCharacter.MCSCharacter_C|GetAttackDirection (Variables|References|GetAIPawn)) "NewEnumerator6")
      (Variables|/Game/MCS/Blueprints/MCSCharacter.MCSCharacter_C|SetAttackDirection (Variables|References|GetAIPawn) "NewEnumerator5")
      (elif (Utilities|Enum|Equal(Enum) (Variables|/Game/MCS/Blueprints/MCSCharacter.MCSCharacter_C|GetAttackDirection (Variables|References|GetAIPawn)) "NewEnumerator5")
        (Variables|/Game/MCS/Blueprints/MCSCharacter.MCSCharacter_C|SetAttackDirection (Variables|References|GetAIPawn) "NewEnumerator6")))))

(fn SelectRandomRollDirection
  (switch int (Math|Random|RandomIntegerinRange 0 2)
    (:0
      (LocalVariables|SetDirection "NewEnumerator7")
      (CallFunction|MoveBack false))
    (:1
      (LocalVariables|SetDirection "NewEnumerator5")
      (CallFunction|StrafeRight false))
    (:2
      (LocalVariables|SetDirection "NewEnumerator6")
      (CallFunction|StrafeLeft false)))
  (Variables|/Game/MCS/Blueprints/MCSCharacter.MCSCharacter_C|SetAttackDirection (Variables|References|GetAIPawn) (LocalVariables|GetDirection)))

(fn CasttoAI
  (params (AIController :type AI%20Controller%20Object%20Reference) (Pawn :type Pawn%20Object%20Reference))
  (if (and (Utilities|IsValid AIController) (Utilities|IsValid Pawn))
    (bind _asmcsbot_controller (Utilities|Casting|CastToMCSBotController AIController)
      (:then
        (bind _asmcsbot (Utilities|Casting|CastToMCSBot Pawn)
          (:then
            (return _asmcsbot_controller _asmcsbot))
          (:CastFailed
            (Development|PrintString "MCSBTT_Task: Cast to MCSBot FAILED"))))
      (:CastFailed
        (Development|PrintString "MCSBTT_Task: Cast to MCSBotController FAILED")))))

(fn CasttoEnemy
  (bind _aipawn (Variables|References|GetAIPawn))
  (Utilities|IsValid _aipawn
    (:Is%20Valid
      (Utilities|IsValid (AI|GetBlackboard _aipawn)
        (:Is%20Valid
          (bind _asmcscharacter (Utilities|Casting|CastToMCSCharacter (AI|Components|Blackboard|GetValueasObject (AI|GetBlackboard (Variables|References|GetAIPawn)) (Utilities|Name|MakeLiteralName "closestEnemy")))
            (:then
              (return _asmcscharacter))
            (:CastFailed
              (Development|PrintString "MCSBTT_Task <CastEnemy MACRO>: Cast to MCSCharacter FAILED"))))))))