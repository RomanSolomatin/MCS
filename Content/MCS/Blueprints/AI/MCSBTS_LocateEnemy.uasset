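; Behavior tree service for MCSBot AI that locates the nearest human player as its enemy.
; On each AI tick, it scans actors tagged HumanPlayer, casts them to MCSCharacter and keeps the closest by distance to the bot.
; When one is valid, it writes that character to the enemy blackboard key, along with a freshly rolled random integer in a second key.
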(event EventReceiveTickAI
  (params (OwnerController :type AI%20Controller%20Object%20Reference) (ControlledPawn :type Pawn%20Object%20Reference) (DeltaSeconds :type Float%20%28single-precision%29))
  (bind _asmcsbot_controller (Utilities|Casting|CastToMCSBotController OwnerController))
  (Variables|References|SetAIController _asmcsbot_controller)
  (bind _asmcsbot (Utilities|Casting|CastToMCSBot ControlledPawn))
  (Variables|References|SetAIPawn _asmcsbot)
  (bind _enemyref (CallFunction|FindNearestEnemy))
  (bind _output_get (Variables|References|SetenemyPlayer _enemyref))
  (Utilities|IsValid _output_get
    (:Is%20Valid
      (Class|BTFunctionLibrary|SetBlackboardValueasObject (Variables|BlackboardKeys|GetenemyPlayerKey) (Variables|References|GetenemyPlayer))
      (Class|BTFunctionLibrary|SetBlackboardValueasInt (Variables|BlackboardKeys|GetRandomIntKey) (Math|Random|RandomIntegerinRange 0 100)))))

(fn FindNearestEnemy
  (bind _outactors (Actor|GetAllActorswithTag "HumanPlayer"))
  (for _array_element _outactors
    (bind _asmcscharacter (Utilities|Casting|CastToMCSCharacter _array_element))
    (LocalVariables|SetcurrentEnemy _asmcscharacter)
    (bind _output_get (LocalVariables|SetcurrentDistance (Transformation|GetDistanceTo (Variables|References|GetAIPawn) (LocalVariables|GetcurrentEnemy))))
    (if (< _output_get (LocalVariables|GetnearestDistance))
      (LocalVariables|SetnearestDistance (LocalVariables|GetcurrentDistance))
      (LocalVariables|SetnearestEnemy (LocalVariables|GetcurrentEnemy))))
  (return (LocalVariables|GetnearestEnemy)))