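; MCS Behavior Tree task for AI defending against its target, failing if that target is dead.
; If the AI is not already defending it calls WalkPressed, then reports success either way.
; GetDefendValue maps the target's attack direction to a left, center or right defend value, but the nodes writing it to DefendInfo are disconnected.
; GetLaunchVector builds an upward vector toward the target and is not called here.
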(event EventReceiveExecuteAI
  (params (OwnerController :type AI%20Controller%20Object%20Reference) (ControlledPawn :type Pawn%20Object%20Reference))
  (|CallParentFunction OwnerController ControlledPawn)
  (if (not (Variables|/Game/MCS/Characters/MCSCharacter.MCSCharacter_C|GetIsDead? (Variables|Default|GetTargetRef)))
    (if (not (.IsDefending (Utilities|Struct|BreakMCSDefendInfo (Variables|/Game/MCS/Characters/MCSCharacter.MCSCharacter_C|GetDefendInfo (Variables|Default|GetAICharacterRef)))))
      (Default|WalkPressed (Variables|Default|GetAICharacterRef))
      (AI|BehaviorTree|FinishExecute true)
      (else
        (AI|BehaviorTree|FinishExecute true)))
    (else
      (AI|BehaviorTree|FinishExecute false))))

(fn GetLaunchVector
  (bind _targetref (Variables|Default|GetTargetRef))
  (bind _aicharacterref (Variables|Default|GetAICharacterRef))
  (bind _returnvalue (Transformation|GetActorLocation _targetref))
  (bind _returnvalue_2 (Transformation|GetActorLocation _aicharacterref))
  (bind _returnvalue_3 (- _returnvalue _returnvalue_2))
  (bind (_x _y) (Math|Vector|BreakVector _returnvalue_3))
  (LocalVariables|SetVector (Math|Vector|MakeVector _x _y 1e+03))
  (return (LocalVariables|GetVector)))

(fn GetDefendValue
  (switch Utilities|FlowControl|Switch|SwitchonMCSAttackDirection (.CurrentAttack (Utilities|Struct|BreakMCSAttackInfo (Variables|/Game/MCS/Characters/MCSCharacter.MCSCharacter_C|GetCurrentAttackInfo (Variables|Default|GetTargetRef))))
    (:NewEnumerator8
      (LocalVariables|SetDefendValue 5e+01 :!label _label))
    (:NewEnumerator0
      (goto _label))
    (:NewEnumerator1
      (goto _label))
    (:NewEnumerator2
      (goto _label))
    (:NewEnumerator7
      (goto _label))
    (:NewEnumerator3
      (LocalVariables|SetDefendValue 0.0 :!label _label_2))
    (:NewEnumerator4
      (LocalVariables|SetDefendValue 1e+02 :!label _label_3))
    (:NewEnumerator5
      (goto _label_2))
    (:NewEnumerator6
      (goto _label_3)))
  (return (LocalVariables|GetDefendValue)))