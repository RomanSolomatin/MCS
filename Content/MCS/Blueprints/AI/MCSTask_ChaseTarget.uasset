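; Behavior tree task that chases the combat target for an AI character in the MCS framework.
; Each AI tick, while the character is alive, it smooths speed up to combat speed if stopped and issues an AI MoveTo toward the target at the combat radius.
; It clears the InAttackRange blackboard key while moving, then sets it and finishes successfully on arrival.
; An unconnected branch for random jumps at long distance never runs.
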(event EventReceiveTickAI
  (params (OwnerController :type AI%20Controller%20Object%20Reference) (ControlledPawn :type Pawn%20Object%20Reference) (DeltaSeconds :type Float%20%28single-precision%29))
  (bind _aicharacterref (Variables|Default|GetAICharacterRef))
  (|CallParentFunction OwnerController ControlledPawn DeltaSeconds)
  (if (not (Variables|/Game/MCS/Blueprints/MCSCharacter.MCSCharacter_C|GetIsDead? (Variables|Default|GetAICharacterRef)))
    (if (<= (Variables|Default|GetCurrentSpeed) 0.0)
      (Default|CLIENTSmoothSpeed _aicharacterref (Variables|/Game/MCS/Blueprints/MCSCharacter.MCSCharacter_C|GetDefaultCombatSpeed _aicharacterref) 15.0))
    (AI|AIMoveTo (Variables|Default|GetAICharacterRef) (Variables|Default|GetTargetXYLocation) (Variables|Default|GetTargetRef) (Variables|/Game/MCS/Blueprints/MCSCharacter.MCSCharacter_C|GetDefaultCombatRadius (Variables|Default|GetAICharacterRef)) false
      (:then
        (Class|BTFunctionLibrary|SetBlackboardValueasBool (Variables|Keys|GetInAttackRange) false))
      (:OnSuccess
        (Class|BTFunctionLibrary|SetBlackboardValueasBool (Variables|Keys|GetInAttackRange) true)
        (AI|BehaviorTree|FinishExecute true)))))