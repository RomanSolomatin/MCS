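; Behavior tree service that syncs an MCS AI character's enemy player target to the blackboard.
; On tick it caches the AI controller and pawn, then writes target, distance, both locations and an in-attack-range flag from combat radius plus buffer.
; It also focuses the controller on the target.
; When the enemy reference is invalid, it clears only the target key.
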(event EventReceiveTickAI
  (params (OwnerController :type AI%20Controller%20Object%20Reference) (ControlledPawn :type Pawn%20Object%20Reference) (DeltaSeconds :type Float%20%28single-precision%29))
  (Variables|Globals|SetDeltaSeconds DeltaSeconds)
  (if (!= (Variables|References|GetAIControllerRef) 0)
    _
    (else
      (bind _asmcsaicontroller (Utilities|Casting|CastToMCSAIController OwnerController))
      (bind _output_get (Variables|References|SetAIControllerRef _asmcsaicontroller))
      (bind _asmcscharacter (Utilities|Casting|CastToMCSCharacter (Pawn|GetControlledPawn _output_get)))
      (Variables|References|SetAICharacterRef _asmcscharacter)))
  (Utilities|IsValid (Variables|/Game/MCS/Blueprints/MCSCharacter.MCSCharacter_C|GetEnemyPlayerRef (Variables|References|GetAICharacterRef))
    (:Is%20Valid
      (Variables|References|SetTargetRef (Variables|/Game/MCS/Blueprints/MCSCharacter.MCSCharacter_C|GetEnemyPlayerRef (Variables|References|GetAICharacterRef)))
      (Class|BTFunctionLibrary|SetBlackboardValueasObject (Variables|Keys|GetTargetToFollowKey) (Variables|References|GetTargetRef))
      (bind _output_get_2 (Variables|Target|SetDistanceToTarget (Transformation|GetDistanceTo (Variables|References|GetAICharacterRef) (Variables|References|GetTargetRef))))
      (Class|BTFunctionLibrary|SetBlackboardValueasFloat (Variables|Keys|GetDistanceToTargetKey) _output_get_2)
      (bind _output_get_3 (Variables|AI|SetAILocation (Transformation|GetActorLocation (Variables|References|GetAICharacterRef))))
      (AI|BehaviorTree|SetBlackboardValueasVector (Variables|Keys|GetAILocationKey) _output_get_3)
      (bind _output_get_4 (Variables|Target|SetTargetLocation (Transformation|GetActorLocation (Variables|References|GetTargetRef))))
      (AI|BehaviorTree|SetBlackboardValueasVector (Variables|Keys|GetTargetLocationKey) _output_get_4)
      (AI|SetFocus (Variables|References|GetAIControllerRef) (Variables|References|GetTargetRef))
      (Class|BTFunctionLibrary|SetBlackboardValueasBool (Variables|Keys|GetInAttackRangeKey) (<= (Variables|Target|GetDistanceToTarget) (+ (Variables|/Game/MCS/Blueprints/MCSCharacter.MCSCharacter_C|GetDefaultCombatRadius (Variables|References|GetAICharacterRef)) (Variables|/Game/MCS/Blueprints/MCSCharacter.MCSCharacter_C|GetCombatRadiusBuffer (Variables|References|GetAICharacterRef))))))
    (:Is%20Not%20Valid
      (Class|BTFunctionLibrary|SetBlackboardValueasObject (Variables|Keys|GetTargetToFollowKey)))))