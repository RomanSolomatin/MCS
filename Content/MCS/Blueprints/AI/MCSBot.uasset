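; AI-controlled lightsaber bot character that seeds blackboard defaults and plays a spawn sound.
; AI_Attack fakes a mouse press against the closest living enemy, throttled by a delayed DoOnce reset, driving attacks with stance-based play rates and side-weighted random directions.
; Multicast-named events toggle saber hit detection and feed attack, abort and roll state to the bot AnimBP, alongside a launch-based jump.
; Hit/death sounds, pitch lean and simulated roll input are disconnected.
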(event Custom|BotHasSpawned
  (params (BotLocation :type Vector))
  ;[1 1 1] Play spawn sound for all the clients
  (Audio|PlaySoundatLocation "/Game/MCS/Sounds/Bot/Spawn_Cue.Spawn_Cue" BotLocation))

(event EventCLIENTPlayerSoundonHit
  (params (HitResult :type Hit%20Result%20Structure)))

(event EventTick
  (params (DeltaSeconds :type Float%20%28single-precision%29))
  (|CallParentFunction DeltaSeconds))

(event EventInitSpawn
  (CallFunction|BotHasSpawned (Transformation|GetActorLocation))
  ;[1 1 1] Set any default blackboard values for the AI
  (AI|Components|Blackboard|SetValueasFloat (AI|GetBlackboard self) (Utilities|Name|MakeLiteralName "attackRadius") (Variables|Default|GetDefaultAttackRadius))
  (AI|Components|Blackboard|SetValueasBool (AI|GetBlackboard self) (Utilities|Name|MakeLiteralName "InCombatRange") false)
  (bind _weapon (CallFunction|GetWeapon))
  (Variables|Default|SetWeaponRef _weapon))

(event EventCLIENTPlayerSoundonDeath
  (params (HitResult :type Hit%20Result%20Structure)))

(event EventOnLanded
  (params (Hit :type Hit%20Result%20Structure%20%28by%20ref%29)))

(event Custom|AI_AttackInDirectionMulticast
  (params (Direction :type MCSAttackDirection%20Enum :default "NewEnumerator8"))
  (bind _lightsabercomponent (Variables|Default|GetLightsaberComponent))
  (bind _childactor (Variables|/Script/Engine.ChildActorComponent|GetChildActor _lightsabercomponent))
  ;[1 1 1] AI Attack
  (Variables|Default|SetAttackDirection Direction)
  (if (Variables|Default|GetInCombatMode)
    (if (not (Variables|Default|GetIsAttacking?))
      (Math|Integer|IncrementInt (Variables|Default|GetDelayedComboCount)
        (:%20%20
          (Utilities|IsValid _childactor
            (:Is%20Valid
              (bind _aslightsaber (Utilities|Casting|CastToLightsaber _childactor))
              (Default|EnableHitDetection _aslightsaber true)
              (Variables|Default|SetHitCount 0)
              (Variables|Default|SetAttackTime 0.0)
              (Variables|Default|SetCanStillAttack? false)
              (Variables|Default|SetIsAttacking? true)
              (bind _asmcsbot_animation (Utilities|Casting|CastToMCSBotAnimation (Components|SkeletalMesh|GetAnimInstance (Variables|Character|GetMesh))))
              (Variables|/Game/MCS/Blueprints/MCSAnimation.MCSAnimation_C|SetAttackDirection _asmcsbot_animation (Variables|Default|GetAttackDirection)))))))
    (else
      (Utilities|FlowControl|DoOnce false
        (:Completed
          (CallFunction|SRVToggleCombatMode))))))

(event Custom|AI_RollMulticast
  ;[1 1 1] AI Rolling
  (if (not (Variables|Default|GetIsAttacking?))
    (Variables|Default|SetIsCrouching? true)
    (bind _asmcsbot_animation (Utilities|Casting|CastToMCSBotAnimation (Components|SkeletalMesh|GetAnimInstance (Variables|Character|GetMesh))))
    (Variables|/Game/MCS/Blueprints/MCSAnimation.MCSAnimation_C|SetIsCrouching? _asmcsbot_animation (Variables|Default|GetIsCrouching?))
    (Variables|/Game/MCS/Blueprints/MCSAnimation.MCSAnimation_C|SetAttackDirection _asmcsbot_animation (Variables|Default|GetAttackDirection))
    (Utilities|FlowControl|Delay 0.1)
    (Variables|Default|SetIsCrouching? false)
    (bind _asmcsbot_animation_2 (Utilities|Casting|CastToMCSBotAnimation (Components|SkeletalMesh|GetAnimInstance (Variables|Character|GetMesh))))
    (Variables|/Game/MCS/Blueprints/MCSAnimation.MCSAnimation_C|SetIsCrouching? _asmcsbot_animation_2 (Variables|Default|GetIsCrouching?))))

(event Custom|AI_Walk
  ;[1 1 1] AI Walk/Run
  (if (Variables|Default|GetIsSprinting?)
    (Variables|Default|SetIsSprinting? false)))

(event Custom|AI_AbortAttackMulticast
  ;[1 1 1] AI Attack
  (bind _asmcsbot_animation (Utilities|Casting|CastToMCSBotAnimation (Components|SkeletalMesh|GetAnimInstance (Variables|Character|GetMesh))))
  (Default|AbortAttack _asmcsbot_animation))

(event Custom|AI_AttackMulticast
  (bind _lightsabercomponent (Variables|Default|GetLightsaberComponent))
  (bind _childactor (Variables|/Script/Engine.ChildActorComponent|GetChildActor _lightsabercomponent))
  ;[1 1 1] AI Attack
  (Math|Integer|IncrementInt (Variables|Default|GetDelayedComboCount)
    (:%20%20
      (Utilities|IsValid _childactor
        (:Is%20Valid
          (bind _aslightsaber (Utilities|Casting|CastToLightsaber _childactor))
          (Default|EnableHitDetection _aslightsaber true)
          (Variables|Default|SetHitCount 0)
          (Variables|Default|SetAttackTime 0.0)
          (Variables|Default|SetCanStillAttack? false)
          (Variables|Default|SetIsAttacking? true)
          (bind _direction (CallFunction|GetBotAttackDirection))
          (bind _asmcsbot_animation (Utilities|Casting|CastToMCSBotAnimation (Components|SkeletalMesh|GetAnimInstance (Variables|Character|GetMesh))))
          (Variables|/Game/MCS/Blueprints/MCSAnimation.MCSAnimation_C|SetAttackDirection _asmcsbot_animation _direction))))))

(event Custom|AI_Run
  ;[1 1 1] AI Walk/Run
  (if (Variables|Default|GetIsSprinting?)
    (Variables|Default|SetIsSprinting? true)))

(event Custom|ResetAttack
  (Utilities|FlowControl|DoOnce false) ; enters at Reset
)

(event Custom|BOT_Attack
  (if (Variables|Default|GetInCombatMode)
    (Variables|Default|SetStartTime (Utilities|Time|GetTimeSeconds))
    (if (CallFunction|PlayerCanAttack)
      (bind _output_get (Variables|Default|SetDelayedComboCount 0))
      (Variables|Default|SetChainComboCount _output_get)
      (switch Utilities|FlowControl|Switch|SwitchonMCSCombatStance (Variables|Default|GetCombatStance)
        (:NewEnumerator1
          (Variables|Default|SetCurrentAttackPlayRate (Variables|Default|GetDefaultAttackPlayRateMedium))
          ;[1 0 0] Will be removed when medium is implemented
          (Variables|Default|SetStageModifier 0.25))
        (:NewEnumerator2
          (Variables|Default|SetCurrentAttackPlayRate (Variables|Default|GetDefaultAttackPlayRateHeavy))))
      (bind _direction (CallFunction|SetRandomDirection))
      (bind _output_get_2 (Variables|Default|SetAttackDirection _direction))
      (Utilities|Struct|SetmembersinMCSAttackInfo (Variables|Default|GetCurrentAttackInfo) _output_get_2 _output_get_2 (Variables|Default|GetCurrentAttackPlayRate))
      (CallFunction|CLIENTAttack))
    (else
      (Utilities|Struct|SetmembersinMCSAttackInfo (Variables|Default|GetCurrentAttackInfo))
      (CallFunction|CLIENTToggleCombatMode)
      ;[1 0 0] Debug
      (CallFunction|ShowSwingStage false))))

(event Custom|AI_Attack
  (bind _asmcscharacter (Utilities|Casting|CastToMCSCharacter (AI|Components|Blackboard|GetValueasObject (AI|GetBlackboard self) (Utilities|Name|MakeLiteralName "closestEnemy"))))
  (if (not (Variables|/Game/MCS/Blueprints/MCSCharacter.MCSCharacter_C|GetIsDead? _asmcscharacter))
    (Utilities|FlowControl|DoOnce false
      (:Completed
        (Variables|Default|SetIsMouseDown true)
        (CallFunction|BOTAttack)
        (Variables|Default|SetIsMouseDown false)
        (Utilities|FlowControl|Delay 1.6)
        (CallFunction|ResetAttack)))))

(event Custom|AI_Jump
  (params (Duration :type Float%20%28single-precision%29))
  ;[1 1 1] AI Jumping
  (if (not (AI|Components|NavMovement|IsFalling (Variables|Character|GetCharacterMovement)))
    (Character|LaunchCharacter (* (+ (Transformation|GetActorUpVector) (Transformation|GetActorForwardVector)) 1.25e+03) false false)))

(event EventMULTIAttackEnded
  (bind _lightsabercomponent (Variables|Default|GetLightsaberComponent))
  (bind _childactor (Variables|/Script/Engine.ChildActorComponent|GetChildActor _lightsabercomponent))
  ;[1 1 1] AI Attack
  (Variables|Default|SetIsAttacking? false)
  (Variables|Default|SetIsRecovering? false)
  (Variables|Default|SetDelayedComboCount 0)
  (Variables|Default|SetCombatStance "NewEnumerator2")
  (Variables|Default|SetAttackTime 0.0)
  (Variables|Default|SetHitCount 0)
  (Utilities|IsValid _childactor
    (:Is%20Valid
      (bind _aslightsaber (Utilities|Casting|CastToLightsaber _childactor))
      (Default|EnableHitDetection _aslightsaber false))))

(fn ConstructionScript
  (|CallParentFunction))

(fn RollRightLeft
  (params (Speed :type Float%20%28single-precision%29))
  (Transformation|SetActorLocation (+ (Transformation|GetActorLocation) (* (Transformation|GetActorRightVector) (* (Variables|Default|GetDeltaSeconds) Speed))) false false)
  (return))

(fn GetBotAttackDirection
  (switch Utilities|FlowControl|Switch|SwitchonMCSAttackDirection (Variables|Default|GetAttackDirection)
    (:NewEnumerator8
      (switch int (Math|Random|RandomIntegerinRange 0 6) :!label _label
        (:0
          (Variables|Default|SetBotAttackDirection "NewEnumerator0"))
        (:1
          (Variables|Default|SetBotAttackDirection "NewEnumerator5"))
        (:2
          (Variables|Default|SetBotAttackDirection "NewEnumerator5"))
        (:3
          (Variables|Default|SetBotAttackDirection "NewEnumerator5"))
        (:4
          (Variables|Default|SetBotAttackDirection "NewEnumerator6"))
        (:5
          (Variables|Default|SetBotAttackDirection "NewEnumerator6"))))
    (:NewEnumerator0
      (goto _label))
    (:NewEnumerator5
      (switch int (Math|Random|RandomIntegerinRange 0 2)
        (:0
          (Variables|Default|SetBotAttackDirection "NewEnumerator5"))
        (:1
          (Variables|Default|SetBotAttackDirection "NewEnumerator5"))
        (:2
          (Variables|Default|SetBotAttackDirection "NewEnumerator2"))))
    (:NewEnumerator6
      (switch int (Math|Random|RandomIntegerinRange 0 2)
        (:0
          (Variables|Default|SetBotAttackDirection "NewEnumerator6"))
        (:1
          (Variables|Default|SetBotAttackDirection "NewEnumerator6"))
        (:2
          (Variables|Default|SetBotAttackDirection "NewEnumerator2")))))
  (return (Variables|Default|GetBotAttackDirection)))

(fn RollForward
  (params (Speed :type Float%20%28single-precision%29))
  (Transformation|SetActorLocation (+ (Transformation|GetActorLocation) (* (Transformation|GetActorForwardVector) (* (Variables|Default|GetDeltaSeconds) Speed))) false false)
  (return))

(fn GetWeapon
  (bind _lightsabercomponent (Variables|Default|GetLightsaberComponent))
  (bind _childactor (Variables|/Script/Engine.ChildActorComponent|GetChildActor _lightsabercomponent))
  (Utilities|IsValid _childactor
    (:Is%20Valid
      (bind _aslightsaber (Utilities|Casting|CastToLightsaber _childactor))
      (return _aslightsaber))))

(fn SetRandomDirection
  (switch int (Math|Random|RandomIntegerinRange 0 6)
    (:0
      (Variables|Default|SetBotAttackDirection "NewEnumerator0"))
    (:1
      (Variables|Default|SetBotAttackDirection "NewEnumerator5"))
    (:2
      (Variables|Default|SetBotAttackDirection "NewEnumerator5"))
    (:3
      (Variables|Default|SetBotAttackDirection "NewEnumerator5"))
    (:4
      (Variables|Default|SetBotAttackDirection "NewEnumerator6"))
    (:5
      (Variables|Default|SetBotAttackDirection "NewEnumerator6"))
    (:6
      (Variables|Default|SetBotAttackDirection "NewEnumerator6")))
  (return (Variables|Default|GetBotAttackDirection)))